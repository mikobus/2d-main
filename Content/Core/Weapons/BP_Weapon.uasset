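; BP_Weapon is a weapon actor that takes its visuals from item data and places itself on the game's tile map.
; The construction script looks up the item's data table row and applies its sprite and animated flipbook to the Paper2D weapon components.
; On BeginPlay it waits briefly, gets the tile map from BP_Gamemode and moves to the world location of a hard-coded tile.
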(event EventBeginPlay
  (Utilities|FlowControl|Delay 0.1)
  (bind _asbp_gamemode (Utilities|Casting|CastToBP_Gamemode (Game|GetGameMode)))
  (Variables|Default|SetTile%20Map (Variables|/Game/Core/BP_Gamemode.BP_Gamemode_C|GetTileMap _asbp_gamemode))
  (bind (_tilex _tiley) (Default|TiletoLocation (Variables|Default|GetTile%20Map) 20 4))
  (Transformation|SetActorLocation (Math|Vector|MakeVector _tilex _tiley 0.0) false false))

(fn ConstructionScript
  (bind _itemdata (Variables|Default|GetItemData))
  (bind _returnvalue (Utilities|GetDataTableRow (.datatable (.item _itemdata)) (.rowname (.item _itemdata)))
    (:then
      (Rendering|Components|Sprite|SetSprite (Variables|Default|GetWeapon) (.Mesh (Utilities|Struct|BreakS_Weapon _returnvalue)))
      (Sprite|SetFlipbook (Variables|Default|GetAnimatedWeapon) (.AnimatedWeapon (Utilities|Struct|BreakS_Weapon _returnvalue))))))