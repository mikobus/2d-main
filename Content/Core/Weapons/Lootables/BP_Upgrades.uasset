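; BP_Upgrades is a Paper2D upgrade pickup that opens an upgrade pick UI and raises the character's level.
; Shortly after BeginPlay it gets the tilemap from BP_Gamemode and moves itself to a hardcoded tile.
; On overlap with BP_Character it closes any open pick UI, shows a new PickUI, increments CurrentLevel and destroys itself.
; The construction script stops its flipbook animation.
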(event EventBeginPlay
  (Utilities|FlowControl|Delay 0.2)
  (Utilities|FlowControl|Sequence
    (:then_0
      (bind _asbp_gamemode (Utilities|Casting|CastToBP_Gamemode (Game|GetGameMode)))
      (Variables|Default|SetTile%20Map (Default|GetTIlemap _asbp_gamemode)))
    (:then_1
      (bind (_tilex _tiley) (Default|TiletoLocation (Variables|Default|GetTile%20Map) 20 15))
      (Transformation|SetActorLocation (Math|Vector|MakeVector _tilex _tiley 0.0) false false))))

(event Collision|EventActorBeginOverlap
  (params (OtherActor :type Actor%20Object%20Reference))
  (bind _asbp_character (Utilities|Casting|CastToBP_Character OtherActor))
  (Utilities|IsValid (Variables|/Game/Core/BP_Character.BP_Character_C|GetPickUIReference _asbp_character)
    (:Is%20Valid
      (Default|CloseUI _asbp_character))
    (:Is%20Not%20Valid
      _))
  (bind _returnvalue (Game|ConstructObjectfromClass _asbp_character "/Game/Core/Weapons/Lootables/UpgradesUI/PickUI.PickUI_C"))
  (UserInterface|Viewport|AddtoViewport _returnvalue 0)
  (Variables|/Game/Core/BP_Character.BP_Character_C|SetCurrentLevel _asbp_character (+ (Variables|/Game/Core/BP_Character.BP_Character_C|GetCurrentLevel _asbp_character) 1))
  (Actor|DestroyActor))

(fn ConstructionScript
  (Audio|Components|Audio|Stop (Variables|Default|GetPaperFlipbook)))