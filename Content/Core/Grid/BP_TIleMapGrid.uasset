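; Tile map grid actor that loads a dungeon tile map and makes it editable at BeginPlay.
; LocationToTile converts world positions to tile indices relative to the actor, with X as up/down, Y as left/right and a hardcoded 32-unit divisor.
; TileToLocation maps indices back to world coordinates using TileSize, with its half-tile centering offset switched off.
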(event EventBeginPlay
  (Class|PaperTileMapComponent|SetTileMap (Variables|Default|GetTileMap) "/Game/Core/Tilemaps/tileset_dungeon_TileSet1Map.tileset_dungeon_TileSet1Map")
  (Class|PaperTileMapComponent|MakeTileMapEditable (Variables|Default|GetTileMap)))

(fn ConstructionScript)

(fn LocationtoTile
  (params (Location :type Vector))
  (bind _output_get (Variables|Default|SetLocation Location))
  (bind (_mapwidth _mapheight) (Class|PaperTileMapComponent|GetMapSize (Variables|Default|GetTileMap)))
  (return (/ (Math|Float|Floor (* _mapwidth (/ (- (.x _output_get) (.x (Transformation|GetActorLocation))) _mapwidth))) 32) (/ (Math|Float|Floor (* _mapheight (/ (- (.y _output_get) (.y (Transformation|GetActorLocation))) _mapheight))) 32)))

(fn TiletoLocation
  (params (LEFT/RIGHT :type Integer) (UP/DOWN :type Integer))
  (bind _returnvalue (Transformation|GetActorLocation))
  (bind _tilesize (Variables|Default|GetTileSize))
  (bind _returnvalue_2 (/ _tilesize 2.0))
  (bind _returnvalue_3 (select false _returnvalue_2 0.0))
  (Variables|Default|SetMapWidth UP/DOWN)
  (Variables|Default|SetMapHeight LEFT/RIGHT)
  (return (+ (+ (* (Variables|Default|GetMapWidth) (Variables|Default|GetTileSize)) (.x _returnvalue)) _returnvalue_3) (+ _returnvalue_3 (+ (.y _returnvalue) (* (Variables|Default|GetMapHeight) (Variables|Default|GetTileSize))))))