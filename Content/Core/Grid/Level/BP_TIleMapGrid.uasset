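; Level tile map actor that chains procedurally generated maps as the player progresses.
; When the player overlaps Box, it shows an event UI; MapChosen then clears enemies, spawns a BP_ProceduralTileMap, increments the gamemode level and spawns a level-scaled enemy spawner.
; When the player leaves GateBox, it overwrites two edge tile strips, apparently gateways, and rebuilds collision.
; Helper functions convert between world locations and tile coordinates.
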(event OnComponentBeginOverlap(Box)
  (params (OverlappedComponent :type Primitive%20Component%20Object%20Reference) (OtherActor :type Actor%20Object%20Reference) (OtherComp :type Primitive%20Component%20Object%20Reference) (OtherBodyIndex :type Integer) (bFromSweep :type Boolean) (SweepResult :type Hit%20Result%20Structure%20%28by%20ref%29))
  (if (Utilities|Operators|EqualEqual (Transformation|GetActorLocation OtherActor) (Transformation|GetActorLocation (Game|GetPlayerCharacter 0)) 5.0)
    (Collision|SetCollisionEnabled (Variables|Default|GetBox) "NoCollision")
    (bind _asbp_character (Utilities|Casting|CastToBP_Character OtherActor))
    (bind _returnvalue (Game|ConstructObjectfromClass _asbp_character "/Game/Core/LevelSwitches/TownItems/MapUI/EventUI.EventUI_C"))
    (UserInterface|Viewport|AddtoViewport _returnvalue 0)))

(event OnComponentEndOverlap(GateBox)
  (params (OverlappedComponent :type Primitive%20Component%20Object%20Reference) (OtherActor :type Actor%20Object%20Reference) (OtherComp :type Primitive%20Component%20Object%20Reference) (OtherBodyIndex :type Integer))
  (if (Utilities|Operators|EqualEqual (Transformation|GetActorLocation OtherActor) (Transformation|GetActorLocation (Game|GetPlayerCharacter 0)) 5.0)
    (for _index (range 0 1)
      (for _index_2 (range 19 21)
        (Class|PaperTileMapComponent|SetTile (Variables|Default|GetTileMap) _index_2 _index 3 (Utilities|Struct|MakePaperTileInfo 43 "/Game/Core/Spirtes/Tilesets/Nature/IceTileset_TileSet.IceTileset_TileSet" false false false))))
    (for _index_3 (range 39 40)
      (for _index_4 (range 19 21)
        (Class|PaperTileMapComponent|SetTile (Variables|Default|GetTileMap) _index_4 _index_3 3 (Utilities|Struct|MakePaperTileInfo 43 "/Game/Core/Spirtes/Tilesets/Nature/IceTileset_TileSet.IceTileset_TileSet" false false false))))
    (Class|PaperTileMapComponent|RebuildCollision (Variables|Default|GetTileMap))
    (Components|DestroyComponent (Variables|Default|GetGateBox))))

(event Custom|MapChosen
  (Utilities|IsValid (Variables|Default|GetBox)
    (:Is%20Valid
      (bind _outactors (Actor|GetAllActorsOfClass "/Game/Core/NPC/BP_Enemy.BP_Enemy_C"))
      (for _array_element _outactors
        (Utilities|IsValid _array_element
          (:Is%20Valid
            (Actor|DestroyActor _array_element))))
      (Game|SpawnActorfromClass "/Game/Core/Grid/Level/BP_ProceduralTileMap.BP_ProceduralTileMap_C" (Math|Transform|MakeTransform (Math|Vector|MakeVector (+ (.x (Transformation|GetWorldLocation (Variables|Default|GetBox))) 32.0) 0.0 0.0) "0, 0, 0" "1.000000,1.000000,1.000000") "Undefined" "MultiplyWithRoot" 0 "/Game/Core/Tilemaps/Levels/GENmap.GENmap" (Variables|Default|GetMapType) (Variables|Default|GetTiles) 0)
      (bind _asbp_gamemode (Utilities|Casting|CastToBP_Gamemode (Game|GetGameMode)))
      (bind _output_get (Variables|/Game/Core/BP_Gamemode.BP_Gamemode_C|SetCurrent%20Level _asbp_gamemode (+ (Variables|/Game/Core/BP_Gamemode.BP_Gamemode_C|GetCurrent%20Level _asbp_gamemode) 1)))
      (Game|SpawnActorfromClass "/Game/Core/NPC/Spawners/EnemyTimeSpawner.EnemyTimeSpawner_C" (Math|Transform|MakeTransform "0, 0, 0" "0, 0, 0" "1.000000,1.000000,1.000000") "Undefined" "MultiplyWithRoot" 0 (* _output_get 10) "/Game/Core/NPC/BP_Minotaur.BP_Minotaur_C" _output_get 5.0 0)
      (Widget|RemovefromParent (stale OnComponentBeginOverlap(Box) _returnvalue))
      (Components|DestroyComponent (Variables|Default|GetBox)))))

(event EventBeginPlay
  (bind _tilemap (Variables|Default|GetTileMap))
  (Class|PaperTileMapComponent|SetTileMap (Variables|Default|GetTileMap) (Variables|Default|GetActiveTilemap))
  (Class|PaperTileMapComponent|MakeTileMapEditable _tilemap)
  (Class|PaperTileMapComponent|RebuildCollision _tilemap))

(fn ConstructionScript)

(fn LocationtoTile
  (params (Location :type Vector))
  (bind _mapwidth (Variables|Default|GetMapWidth))
  (bind _mapheight (Variables|Default|GetMapHeight))
  (bind _output_get (Variables|Default|SetLocation Location))
  (return (/ (Math|Float|Floor (* _mapwidth (/ (- (.x _output_get) (.x (Transformation|GetActorLocation))) _mapwidth))) 32) (/ (Math|Float|Floor (* _mapheight (/ (- (.y _output_get) (.y (Transformation|GetActorLocation))) _mapheight))) 32)))

(fn TiletoLocation
  (params (LEFT/RIGHT :type Integer) (UP/DOWN :type Integer))
  (bind _returnvalue (Transformation|GetActorLocation))
  (bind _tilesize (Variables|Default|GetTileSize))
  (bind _returnvalue_2 (/ _tilesize 2.0))
  (bind _returnvalue_3 (select false _returnvalue_2 0.0))
  (Variables|Default|SetMapWidth UP/DOWN)
  (Variables|Default|SetMapHeight LEFT/RIGHT)
  (return (+ (+ (* (Variables|Default|GetMapWidth) (Variables|Default|GetTileSize)) (.x _returnvalue)) _returnvalue_3) (+ _returnvalue_3 (+ (.y _returnvalue) (* (Variables|Default|GetMapHeight) (Variables|Default|GetTileSize))))))