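; BP_Character is the tile-based Paper2D player character, placed via the gamemode's TileMap at BeginPlay alongside its HUD widget.
; Damage updates health with indicators and a red flash; death disables input and runs a camera timeline into burst effects and a death screen.
; Attacks delegate to Inventory, which supplies idle flipbooks and equips a club on Tab.
; Helpers add gold and apply freeze, burn, fear or bleed to enemies.
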(event OnFinishedPlaying(PaperFlipbook)
  ;[0.15 0.15 0.15 0.5] Animation Reset
  (Components|Activation|SetActive (Variables|Default|GetSwingEffect) false true)
  (Sprite|SetFlipbook (Variables|Default|GetPaperFlipbook) (Variables|/Game/Core/Items/GameplayAbilities/BP_WeaponClass.BP_WeaponClass_C|GetIdleStance (Variables|/Game/Core/Inventory.Inventory_C|GetEquippedWeapon (Variables|Default|GetInventory))))
  (Components|Timeline|SetLooping (Variables|Default|GetPaperFlipbook) true)
  (Audio|Components|Audio|Play (Variables|Default|GetPaperFlipbook)))

(event EventBeginPlay
  ;[0.15 0.15 0.15 0.5] Set Starting Tile
  (Utilities|FlowControl|Sequence
    (:then_0
      (bind _asbp_controller (Utilities|Casting|CastToBP_Controller (Pawn|GetController)))
      (bind _asbp_gamemode (Utilities|Casting|CastToBP_Gamemode (Game|GetGameMode)))
      (Variables|References|SetControllerRef _asbp_controller)
      (Variables|Private|SetBPM (Variables|/Game/Core/BP_Gamemode.BP_Gamemode_C|GetBPM _asbp_gamemode))
      (Variables|References|SetAs%20BP%20Gamemode _asbp_gamemode)
      (Variables|References|SetTile%20Map (Variables|/Game/Core/BP_Gamemode.BP_Gamemode_C|GetTileMap _asbp_gamemode))
      (bind _output_get (Variables|/Game/Core/BP_Controller.BP_Controller_C|SetUp/Down _asbp_controller (Variables|Private|GetUp/%20Down%20Start%20Position)))
      (bind _output_get_2 (Variables|/Game/Core/BP_Controller.BP_Controller_C|SetLeft/right _asbp_controller (Variables|Private|GetLeft/right%20Start%20Position)))
      (bind (_tilex _tiley) (Default|TiletoLocation (Variables|References|GetTile%20Map) _output_get_2 _output_get))
      (Transformation|SetActorLocation (Math|Vector|MakeVector _tilex _tiley 0.0) false false))
    (:then_1
      ;[0.15 0.15 0.15 0.5] UI
      (bind _returnvalue (UserInterface|CreateWidget "/Game/Core/Interface/GoldAndUI/I_Interface.I_Interface_C"))
      (Variables|References|SetInterfaceReference _returnvalue)
      (UserInterface|Viewport|AddtoViewport _returnvalue 0))))

(event Game|Damage|EventAnyDamage
  (params (Damage :type Float%20%28single-precision%29) (DamageType :type Damage%20Type%20Object%20Reference) (InstigatedBy :type Controller%20Object%20Reference) (DamageCauser :type Actor%20Object%20Reference))
  (bind _returnvalue (Transformation|GetActorLocation))
  (bind _camera (Variables|Default|GetCamera))
  ;[0.15 0.15 0.15 0.5] Damage Eventand spawn
  (Variables|Default|SetHealth (Math|Float|Truncate (- (Variables|Default|GetHealth) Damage)))
  (Game|SpawnActorfromClass "/Game/Core/Interface/DamageIndicators/BP_DamageInd.BP_DamageInd_C" (Math|Transform|MakeTransform (Transformation|GetActorLocation) "0, 0, 0" "1.000000,1.000000,1.000000") "Undefined" "MultiplyWithRoot" 0 Damage "-" (Variables|Default|GetColor) "" 5e+01 0)
  (Variables|/Script/UMG.Widget|SetVisibility (Variables|/Game/Core/Interface/GoldAndUI/I_Interface.I_Interface_C|GetDamageOutline (Variables|References|GetInterfaceReference)) "Visible")
  (Sprite|SetSpriteColor (Variables|Default|GetPaperFlipbook) "(R=1.000000,G=0.008526,B=0.000000,A=1.000000)")
  (Utilities|FlowControl|Delay 0.2)
  (Sprite|SetSpriteColor (Variables|Default|GetPaperFlipbook) "(R=0.976708,G=1.000000,B=0.989687,A=1.000000)")
  (Variables|/Script/UMG.Widget|SetVisibility (Variables|/Game/Core/Interface/GoldAndUI/I_Interface.I_Interface_C|GetDamageOutline (Variables|References|GetInterfaceReference)) "Hidden")
  (Rendering|Components|TextRender|SetText (Variables|/Game/Core/Interface/GoldAndUI/I_Interface.I_Interface_C|GetHealth (Variables|References|GetInterfaceReference)) (Utilities|Text|ToText(Integer) (Variables|Default|GetHealth)))
  (if (<= (Variables|Default|GetHealth) 0)
    (Input|DisableInput (Game|GetPlayerController 0) 0)
    (Transformation|SetRelativeLocation (Variables|Default|GetPaperFlipbook) "0.000000,0.000000,20.000000" false false)
    (bind _fovtimeline (Timeline|Timeline Play)
      (:Update
        (Camera|SetFieldOfView _camera _fovtimeline)
        (Transformation|SetRelativeLocation _camera "430.000000,0.000000,-200.000000" false false)
        (Audio|Components|Audio|Stop (Variables|Default|GetPaperFlipbook))
        (Widget|RemovefromParent (Variables|References|GetInterfaceReference))
        (Utilities|FlowControl|Delay 0.5)
        (Rendering|ToggleVisibility (Variables|Default|GetPaperFlipbook) true)
        (Niagara|SpawnSystematLocation "/Game/Core/assets/Effects/BloodBurst.BloodBurst" _returnvalue)
        (Game|SpawnActorfromClass "/Game/Core/assets/Effects/BP_BloodDecal.BP_BloodDecal_C" (Math|Transform|MakeTransform _returnvalue (Math|Rotator|MakeRotator (Math|Random|RandomFloatinRange 0.0 1e+01) (Math|Random|RandomFloatinRange 0.0 1e+01) (Math|Random|RandomFloatinRange 0.0 3.6e+02)) "1.000000,1.000000,1.000000") "Undefined" "MultiplyWithRoot" 0 0)
        (Niagara|SpawnSystematLocation "/Game/Core/assets/Effects/CoinBurst.CoinBurst" _returnvalue)
        (bind _returnvalue_2 (Game|ConstructObjectfromClass "/Game/Core/Interface/Death/WB_DeathInterface.WB_DeathInterface_C"))
        (UserInterface|Viewport|AddtoViewport _returnvalue_2 0)))))

(event Input|KeyboardEvents|Tab
  (params (Key :type Key%20Structure :default "None"))
  (:Pressed
    (Utilities|FlowControl|DoOnce false
      (:Completed
        (bind _returnvalue (Game|SpawnActorfromClass "/Game/Core/Items/GameplayAbilities/BP_ClubWeapon.BP_ClubWeapon_C" (Math|Transform|MakeTransform "0, 0, 0" "0, 0, 0" "1.000000,1.000000,1.000000") "Undefined" "MultiplyWithRoot" 0 0))
        (Default|Equip (Variables|Default|GetInventory) _returnvalue false)))))

(fn ConstructionScript)

(fn Attack
  (Default|UseWeapon (Variables|Default|GetInventory) false))

(fn CancelAttack
  (params (CancelBlock? :type Boolean))
  (Variables|Bool|SetChargingAttack false))

(fn AddGold
  (params (goldQuantity :type Integer))
  (bind _returnvalue (Transformation|GetActorLocation))
  (Widget|SetVisibility (Variables|/Game/Core/Interface/GoldAndUI/I_Interface.I_Interface_C|GetaddedGoldText (Variables|References|GetInterfaceReference)) "Visible")
  (Variables|Default|SetGold%20Quantity goldQuantity)
  (Variables|Default|SettotalGold (+ goldQuantity (Variables|Default|GettotalGold)))
  (Game|SpawnActorfromClass "/Game/Core/Interface/DamageIndicators/BP_DamageInd.BP_DamageInd_C" (Math|Transform|MakeTransform (Math|Vector|MakeVector (+ (.x _returnvalue) (Math|Random|RandomIntegerinRange -10 10)) (.y _returnvalue) (.z _returnvalue)) "0, 0, 0" "1.000000,1.000000,1.000000") "Undefined" "MultiplyWithRoot" 0 (Math|Conversions|ToFloat(Integer) goldQuantity) "+" (LocalVariables|GetNewLocalVar) " gold!" 2e+01 0))

(fn CloseUI
  (Widget|RemovefromParent (Variables|References|GetPickUIReference)))

(fn StatusEffects
  (params (Object :type Actor%20Object%20Reference))
  (bind _asbp_enemy (Utilities|Casting|CastToBP_Enemy Object))
  (Utilities|IsValid _asbp_enemy
    (:Is%20Valid
      (Utilities|FlowControl|Sequence
        (:then_0
          (if (Variables|StatusEffects|GetFreezingAttacks)
            (Variables|/Game/Core/NPC/BP_Enemy.BP_Enemy_C|SetFrozen? _asbp_enemy true)
            (Variables|/Game/Core/NPC/BP_Enemy.BP_Enemy_C|SetCrowdControlled? _asbp_enemy true)
            (Rendering|SetVisibility (Variables|/Game/Core/NPC/BP_Enemy.BP_Enemy_C|GetFrozenEffect _asbp_enemy) true false)))
        (:then_1
          (if (Variables|StatusEffects|GetBurningAttacks)
            (Variables|/Game/Core/NPC/BP_Enemy.BP_Enemy_C|SetBurning? _asbp_enemy true)
            (Rendering|SetVisibility (Variables|/Game/Core/NPC/BP_Enemy.BP_Enemy_C|GetBurningEffect _asbp_enemy) true false)
            (Variables|/Game/Core/NPC/BP_Enemy.BP_Enemy_C|SetCrowdControlled? _asbp_enemy true)))
        (:then_2
          (if (Variables|StatusEffects|GetFearAttack)
            (Variables|/Game/Core/NPC/BP_Enemy.BP_Enemy_C|SetFeared? _asbp_enemy true)
            (Variables|/Game/Core/NPC/BP_Enemy.BP_Enemy_C|SetRunChase _asbp_enemy -1)
            (Rendering|SetVisibility (Variables|/Game/Core/NPC/BP_Enemy.BP_Enemy_C|GetFearEffect _asbp_enemy) true false)
            (Variables|/Game/Core/NPC/BP_Enemy.BP_Enemy_C|SetCrowdControlled? _asbp_enemy true)))
        (:then_3
          (if (Variables|StatusEffects|GetBleedAttack)
            (Variables|/Game/Core/NPC/BP_Enemy.BP_Enemy_C|SetBleeding? _asbp_enemy true)
            (Rendering|SetVisibility (Variables|/Game/Core/NPC/BP_Enemy.BP_Enemy_C|GetBleedingEffect _asbp_enemy) true false)
            (Variables|/Game/Core/NPC/BP_Enemy.BP_Enemy_C|SetCrowdControlled? _asbp_enemy true)))))))