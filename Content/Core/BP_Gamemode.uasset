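; Game mode that holds shared run state: the tile map grid, beat interval, current level, and upgrade and event lists.
; BeginPlay caches the first BP_TIleMapGrid, converts BPM to seconds per beat, and fills Upgrades and Events from DataTable row names.
; EventBarFull raises the level and spawns a BP_Chest at the player's horizontal position.
; GetTIlemap exposes the grid; GetEnemyMovement is empty, and enemy spawner scaling is unwired.
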(event Custom|EventBarFull
  (bind _returnvalue (Game|GetPlayerCharacter 0))
  (bind _returnvalue_2 (Transformation|GetActorLocation _returnvalue))
  (bind _output_get (Variables|Default|SetCurrent%20Level (+ (Variables|Default|GetCurrent%20Level) 1)))
  (Development|PrintString (Utilities|String|Append "Current Level: " (Utilities|String|ToString(Integer) _output_get)))
  (Game|SpawnActorfromClass "/Game/Core/Weapons/Lootables/BP_Chest.BP_Chest_C" (Math|Transform|MakeTransform (Math|Vector|MakeVector (.x _returnvalue_2) (.y _returnvalue_2) 5.0) "0, 0, 0" "1.000000,1.000000,1.000000") "Undefined" "MultiplyWithRoot" 0 0))

(event EventBeginPlay
  (bind _outactors (Actor|GetAllActorsOfClass "/Game/Core/Grid/Level/BP_TIleMapGrid.BP_TIleMapGrid_C"))
  (Variables|Default|SetTileMap (Utilities|Array|Get(acopy) _outactors))
  (Variables|Default|SetBPM (/ 6e+01 (Variables|Default|GetBPM)))
  (bind _outrownames (DataTable|GetDataTableRowNames "/Game/Core/Weapons/Lootables/UpgradesUI/Upgrades_DTBaseStats.Upgrades_DTBaseStats"))
  (Variables|Default|SetUpgrades _outrownames)
  (bind _outrownames_2 (DataTable|GetDataTableRowNames "/Game/Core/LevelSwitches/TownItems/MapUI/DT_Maps.DT_Maps"))
  (Variables|Default|SetEvents _outrownames_2))

(fn ConstructionScript)

(fn GetTIlemap
  (return (Variables|Default|GetTileMap)))

(fn GetEnemyMovement)