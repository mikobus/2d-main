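; BP_DebtCollector is a world actor that drains the game's current debt while the player stands in its box.
; On begin play it moves to a fixed tile location from the gamemode's TileMap.
; Box overlap starts and stops a looping PayDebt timer that lowers debt one unit per tick.
; Debt drops even without gold; when the player has gold, each tick also deducts one and spawns BP_PaymentGold targeting the collector.
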(event OnComponentBeginOverlap(Box)
  (params (OverlappedComponent :type Primitive%20Component%20Object%20Reference) (OtherActor :type Actor%20Object%20Reference) (OtherComp :type Primitive%20Component%20Object%20Reference) (OtherBodyIndex :type Integer) (bFromSweep :type Boolean) (SweepResult :type Hit%20Result%20Structure%20%28by%20ref%29))
  (if (== OtherComp (Variables|/Script/Engine.Character|GetCapsuleComponent (Game|GetPlayerCharacter 0)))
    (Utilities|Time|SetTimerbyFunctionName 0 "PayDebt" 0.1 true false 0.5)))

(event OnComponentEndOverlap(Box)
  (params (OverlappedComponent :type Primitive%20Component%20Object%20Reference) (OtherActor :type Actor%20Object%20Reference) (OtherComp :type Primitive%20Component%20Object%20Reference) (OtherBodyIndex :type Integer))
  (if (== OtherComp (Variables|/Script/Engine.Character|GetCapsuleComponent (Game|GetPlayerCharacter 0)))
    (Utilities|Time|ClearTimerbyFunctionName 0 "PayDebt")))

(event EventBeginPlay
  (Utilities|FlowControl|Delay 0.1)
  (bind _asbp_gamemode (Utilities|Casting|CastToBP_Gamemode (Game|GetGameMode)))
  (Variables|Default|SetTile%20Map (Variables|/Game/Core/BP_Gamemode.BP_Gamemode_C|GetTileMap _asbp_gamemode))
  (bind (_tilex _tiley) (Default|TiletoLocation (Variables|Default|GetTile%20Map) 20 10))
  (Transformation|SetActorLocation (Math|Vector|MakeVector _tilex _tiley 0.0) false false))

(fn ConstructionScript)

(fn PayDebt
  (bind _asbp_gamemode (Utilities|Casting|CastToBP_Gamemode (Game|GetGameMode)))
  (if (> (Variables|/Game/Core/BP_Gamemode.BP_Gamemode_C|GetCurrentDebt _asbp_gamemode) 0)
    (Variables|/Game/Core/BP_Gamemode.BP_Gamemode_C|SetCurrentDebt _asbp_gamemode (- (Variables|/Game/Core/BP_Gamemode.BP_Gamemode_C|GetCurrentDebt _asbp_gamemode) 1))
    (bind _asbp_character (Utilities|Casting|CastToBP_Character (Game|GetPlayerCharacter 0)))
    (if (> (Variables|/Game/Core/BP_Character.BP_Character_C|GettotalGold _asbp_character) 0)
      (Variables|/Game/Core/BP_Character.BP_Character_C|SettotalGold _asbp_character (- (Variables|/Game/Core/BP_Character.BP_Character_C|GettotalGold _asbp_character) 1))
      (Game|SpawnActorfromClass "/Game/Core/Interface/GoldAndUI/Blueprints/BP_PaymentGold.BP_PaymentGold_C" (Math|Transform|MakeTransform (Transformation|GetActorLocation (Game|GetPlayerCharacter 0)) "0, 0, 0" "1.000000,1.000000,1.000000") "Undefined" "MultiplyWithRoot" 0 (Transformation|GetActorLocation) 0))))