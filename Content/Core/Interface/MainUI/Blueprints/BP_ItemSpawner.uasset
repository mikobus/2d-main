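; BP_ItemSpawner is an actor built to scatter gold or other objects across a dungeon tilemap, though its event graph logic is disconnected and never runs.
; The unwired logic uses a player-triggered box to swap a tile and start a timer that box-traces random tiles for free space until the count runs out.
; Helper functions spawn either the chosen class or BP_Gold filled from a random item DataTable row.
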(event OnComponentBeginOverlap(Box)
  (params (OverlappedComponent :type Primitive%20Component%20Object%20Reference) (OtherActor :type Actor%20Object%20Reference) (OtherComp :type Primitive%20Component%20Object%20Reference) (OtherBodyIndex :type Integer) (bFromSweep :type Boolean) (SweepResult :type Hit%20Result%20Structure%20%28by%20ref%29))
  ;[0.15 0.15 0.15 0.5] Actor Spawn Loop
  ;;[0.15 0.15 0.15 0.5] open the door
)

(event Custom|Spawn
  ;[0.15 0.15 0.15 0.5] Actor Spawn Loop
)

(event EventBeginPlay
  ;[0.15 0.15 0.15 0.5] Timer
)

(fn ConstructionScript)

(fn SpawnNormalObject
  (params (Tile%20X :type Float%20%28double-precision%29) (Tile%20Y :type Float%20%28double-precision%29))
  ;[0.15 0.15 0.15 0.5] Spawn Normal Object (weapon, equip..)
  (Game|SpawnActorfromClass (Variables|Default|GetClassToSpawn) (Math|Transform|MakeTransform (Math|Vector|MakeVector Tile%20X Tile%20Y 5.0) "0, 0, 0" "1.000000,1.000000,1.000000") "Undefined" "MultiplyWithRoot" 0 0))

(fn SpawnItemObject
  (params (Tile%20X :type Float%20%28double-precision%29) (Tile%20Y :type Float%20%28double-precision%29))
  (bind _dt_items (Variables|Default|GetDT_Items))
  ;[0.15 0.15 0.15 0.5] Spawn Item Object (gold, charm...)
  ;;[0.15 0.15 0.15 0.5] get all possible items (DT rows)
  (bind _outrownames (DataTable|GetDataTableRowNames _dt_items))
  ;;[0.15 0.15 0.15 0.5] get row of random item
  (bind _returnvalue (Utilities|GetDataTableRow _dt_items (.OutItem (Utilities|Array|Random _outrownames)))
    (:then
      (Game|SpawnActorfromClass "/Game/Core/Interface/MainUI/Blueprints/BP_Gold.BP_Gold_C" (Math|Transform|MakeTransform (Math|Vector|MakeVector Tile%20X Tile%20Y 5.0) "0, 0, 0" "1.000000,1.000000,1.000000") "Undefined" "MultiplyWithRoot" 0 _returnvalue (.animation (Utilities|Struct|BreakS_Item _returnvalue)) (Math|Random|RandomIntegerinRange 1 10) 0)
      ;;[0.15 0.15 0.15 0.5] get item type
      (switch Utilities|FlowControl|Switch|SwitchonE_ItemTypes (.BP_type (Utilities|Struct|BreakS_Item _returnvalue))))))