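; BP_Gold is a gold pickup that plays a flipbook animation and pays its value to the player on touch.
; When the player's capsule overlaps its box and the item type is gold, it adds the gold, disables collision and hides the HUD's added-gold text.
; The item then eases quickly toward the player before a pickup sound plays and the actor is destroyed.
; A goods-item type check exists but does nothing.
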(event OnComponentBeginOverlap(Box)
  (params (OverlappedComponent :type Primitive%20Component%20Object%20Reference) (OtherActor :type Actor%20Object%20Reference) (OtherComp :type Primitive%20Component%20Object%20Reference) (OtherBodyIndex :type Integer) (bFromSweep :type Boolean) (SweepResult :type Hit%20Result%20Structure%20%28by%20ref%29))
  (if (== OtherComp (Variables|/Script/Engine.Character|GetCapsuleComponent (Game|GetPlayerCharacter 0)))
    (bind _asbp_character (Utilities|Casting|CastToBP_Character OtherActor))
    (bind _isgold (CallFunction|IsGold))
    (if _isgold
      ;[0.15 0.15 0.15 0.5] add new gold to the player
      (Default|AddGold _asbp_character (Variables|Default|GetValue))
      (Collision|SetCollisionEnabled (Variables|Default|GetBox self) "NoCollision")
      ;;[0.15 0.15 0.15 0.5] hide added gold text
      (Widget|SetVisibility (Variables|/Game/Core/Interface/GoldAndUI/I_Interface.I_Interface_C|GetaddedGoldText (Variables|/Game/Core/BP_Character.BP_Character_C|GetInterfaceReference _asbp_character)) "Hidden")
      (Components|MoveComponentTo (Variables|Default|Getitem) (- (Transformation|GetActorLocation (Game|GetPlayerCharacter 0)) (Transformation|GetActorLocation)) "0, 0, 0" true false 0.1 true)
      (Audio|PlaySound2D "/Game/Core/assets/Audio/UISounds/money-pickup-2-89563.money-pickup-2-89563" 1.0 1.0 0.0 0 0)
      (Actor|DestroyActor)
      (else
        (bind _isgold_2 (CallFunction|IsGoodsItem))
        (if _isgold_2
          _)))))

(event EventBeginPlay
  (Sprite|SetFlipbook (Variables|Default|Getanimation) (Variables|Default|GetFlipbook)))

(fn ConstructionScript)

(fn IsGold
  (return (Utilities|Enum|Equal(Enum) (.BP_type (Utilities|Struct|BreakS_Item (Variables|Default|GetItemData))) "NewEnumerator0")))

(fn IsGoodsItem
  (return (Utilities|Enum|Equal(Enum) (.BP_type (Utilities|Struct|BreakS_Item (Variables|Default|GetItemData))) "NewEnumerator2")))