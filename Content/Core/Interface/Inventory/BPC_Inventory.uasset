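; Inventory actor component that, as it stands, only creates the inventory UI widget on BeginPlay, stores it and adds it to the viewport.
; Unconnected graphs hold logic to toggle the UI and cursor, and to sphere-trace for nearby weapons that get equipped or stored.
; AddWeapon is an empty stub, with its nine-slot limit check, array add and UI refresh left unwired.
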(event EventBeginPlay
  (bind _returnvalue (UserInterface|CreateWidget "/Game/Core/Interface/Inventory/InventoryUI.InventoryUI_C"))
  (bind _output_get (Variables|Default|SetInventoryReference _returnvalue))
  (UserInterface|Viewport|AddtoViewport _output_get 0))

(event Input|KeyboardEvents|Tab
  (params (Key :type Key%20Structure)))

(event Input|KeyboardEvents|E
  (params (Key :type Key%20Structure)))

(event Input|KeyboardEvents|Escape
  (params (Key :type Key%20Structure)))

(fn AddWeapon
  (params (NewWeapon :type S%20Slots%20Structure%20%28by%20ref%29)))