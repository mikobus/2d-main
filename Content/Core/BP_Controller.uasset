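; Player controller for turn-based grid movement and attacks, taking directional Enhanced Input and the Space bar.
; Directions step the character across the TileMap after a line-trace blockage check; while an attack is marked they re-aim it, and pressing the aimed direction cancels it and moves.
; Each successful step or Space attack press calls MovementTick on every BP_Enemy, so enemies act in lockstep.
; AttackMove repeats tile steps along the attack's facing for weapon-driven movement.
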(event Custom|MoveForward
  (bind _up_down (Variables|Default|GetUp/Down))
  (bind _left_right (Variables|Default|GetLeft/right))
  (bind _returnvalue (+ _up_down 1.0))
  (bind _returnvalue_2 (+ _left_right 0.0))
  ;[0.15 0.15 0.15 0.5] Movement
  (if (Utilities|Operators|EqualEqual :A (Variables|/Script/Engine.SceneComponent|GetRelativeRotation (Variables|/Game/Core/BP_Character.BP_Character_C|GetSplineMesh (Variables|Default|GetCharacterReference))))
    (Variables|Default|SetChangingAttack? true))
  (if (Variables|/Game/Core/BP_Character.BP_Character_C|GetAttackMarked (Variables|Default|GetCharacterReference))
    (bind _output_get (Variables|Default|SetAttackDirection 0))
    (if (Variables|Default|GetChangingAttack?)
      (Variables|Default|SetChangingAttack? false :!label _label)
      (Default|CancelAttack (Variables|Default|GetCharacterReference) true)
      (bind _valid_ (Utilities|TileValid? _returnvalue _returnvalue_2)
        (:truth%20exe
          (if _valid_
            (CallFunction|MoveCharacter _returnvalue _returnvalue_2)
            (bind _outactors (Actor|GetAllActorsOfClass "/Game/Core/NPC/BP_Enemy.BP_Enemy_C"))
            (bind _arrayelement (Utilities|Array|ReverseforEachLoop _outactors)
              (:LoopBody
                (Utilities|IsValid _arrayelement
                  (:Is%20Valid
                    (Default|MovementTick _arrayelement))))))))
      (else
        (Transformation|SetRelativeLocationAndRotation (Variables|/Game/Core/BP_Character.BP_Character_C|GetSplineMesh (Variables|Default|GetCharacterReference)) (Utilities|Array|Get(acopy) (Variables|Default|GetAttackVector) _output_get) (Utilities|Array|Get(acopy) (Variables|Default|GetAttackRotation) _output_get) false false)))
    (else
      (goto _label))))

(event Custom|MoveLeft
  (bind _up_down (Variables|Default|GetUp/Down))
  (bind _left_right (Variables|Default|GetLeft/right))
  (bind _returnvalue (+ _up_down 0.0))
  (bind _returnvalue_2 (+ _left_right -1.0))
  ;[0.15 0.15 0.15 0.5] Movement
  (Utilities|Rotate "1.000000,-1.000000,8.000000" "0.000000,-90.000000,90.000000"
    (:NewParam2
      (if (Utilities|Operators|EqualEqual (Variables|/Script/Engine.SceneComponent|GetRelativeRotation (Variables|/Game/Core/BP_Character.BP_Character_C|GetSplineMesh (Variables|Default|GetCharacterReference))) "0.000000,270.000000,0.000000" 0.0)
        (Variables|Default|SetChangingAttack? true))
      (if (Variables|/Game/Core/BP_Character.BP_Character_C|GetAttackMarked (Variables|Default|GetCharacterReference))
        (bind _output_get (Variables|Default|SetAttackDirection 1))
        (if (Variables|Default|GetChangingAttack?)
          (Variables|Default|SetChangingAttack? false :!label _label)
          (Default|CancelAttack (Variables|Default|GetCharacterReference) true)
          (bind _valid_ (Utilities|TileValid? _returnvalue _returnvalue_2)
            (:truth%20exe
              (if _valid_
                (CallFunction|MoveCharacter _returnvalue _returnvalue_2)
                (bind _outactors (Actor|GetAllActorsOfClass "/Game/Core/NPC/BP_Enemy.BP_Enemy_C"))
                (bind _arrayelement (Utilities|Array|ReverseforEachLoop _outactors)
                  (:LoopBody
                    (Utilities|IsValid _arrayelement
                      (:Is%20Valid
                        (Default|MovementTick _arrayelement))))))))
          (else
            (Transformation|SetRelativeLocationAndRotation (Variables|/Game/Core/BP_Character.BP_Character_C|GetSplineMesh (Variables|Default|GetCharacterReference)) (Utilities|Array|Get(acopy) (Variables|Default|GetAttackVector) _output_get) (Utilities|Array|Get(acopy) (Variables|Default|GetAttackRotation) _output_get) false false)))
        (else
          (goto _label))))))

(event Custom|MoveRight
  (bind _up_down (Variables|Default|GetUp/Down))
  (bind _left_right (Variables|Default|GetLeft/right))
  (bind _returnvalue (+ _up_down 0.0))
  (bind _returnvalue_2 (+ _left_right 1.0))
  ;[0.15 0.15 0.15 0.5] Movement
  (Utilities|Rotate "1.000000,1.000000,8.000000" "180.000000,-90.000000,90.000000"
    (:NewParam2
      (if (Utilities|Operators|EqualEqual (Variables|/Script/Engine.SceneComponent|GetRelativeRotation (Variables|/Game/Core/BP_Character.BP_Character_C|GetSplineMesh (Variables|Default|GetCharacterReference))) "0.000000,90.000000,0.000000" 0.0)
        (Variables|Default|SetChangingAttack? true))
      (if (Variables|/Game/Core/BP_Character.BP_Character_C|GetAttackMarked (Variables|Default|GetCharacterReference))
        (bind _output_get (Variables|Default|SetAttackDirection 2))
        (if (Variables|Default|GetChangingAttack?)
          (Variables|Default|SetChangingAttack? false :!label _label)
          (Default|CancelAttack (Variables|Default|GetCharacterReference) true)
          (bind _valid_ (Utilities|TileValid? _returnvalue _returnvalue_2)
            (:truth%20exe
              (if _valid_
                (CallFunction|MoveCharacter _returnvalue _returnvalue_2)
                (bind _outactors (Actor|GetAllActorsOfClass "/Game/Core/NPC/BP_Enemy.BP_Enemy_C"))
                (bind _arrayelement (Utilities|Array|ReverseforEachLoop _outactors)
                  (:LoopBody
                    (Utilities|IsValid _arrayelement
                      (:Is%20Valid
                        (Default|MovementTick _arrayelement))))))))
          (else
            (Transformation|SetRelativeLocationAndRotation (Variables|/Game/Core/BP_Character.BP_Character_C|GetSplineMesh (Variables|Default|GetCharacterReference)) (Utilities|Array|Get(acopy) (Variables|Default|GetAttackVector) _output_get) (Utilities|Array|Get(acopy) (Variables|Default|GetAttackRotation) _output_get) false false)))
        (else
          (goto _label))))))

(event Custom|MoveBack
  (bind _up_down (Variables|Default|GetUp/Down))
  (bind _left_right (Variables|Default|GetLeft/right))
  (bind _returnvalue (+ _up_down -1.0))
  (bind _returnvalue_2 (+ _left_right 0.0))
  ;[0.15 0.15 0.15 0.5] Movement
  (if (Utilities|Operators|EqualEqual (Variables|/Script/Engine.SceneComponent|GetRelativeRotation (Variables|/Game/Core/BP_Character.BP_Character_C|GetSplineMesh (Variables|Default|GetCharacterReference))) "0.000000,180.000000,0.000000" 0.0)
    (Variables|Default|SetChangingAttack? true))
  (if (Variables|/Game/Core/BP_Character.BP_Character_C|GetAttackMarked (Variables|Default|GetCharacterReference))
    (bind _output_get (Variables|Default|SetAttackDirection 3))
    (if (Variables|Default|GetChangingAttack?)
      (Variables|Default|SetChangingAttack? false :!label _label)
      (Default|CancelAttack (Variables|Default|GetCharacterReference) true)
      (bind _valid_ (Utilities|TileValid? _returnvalue _returnvalue_2)
        (:truth%20exe
          (if _valid_
            (CallFunction|MoveCharacter _returnvalue _returnvalue_2)
            (bind _outactors (Actor|GetAllActorsOfClass "/Game/Core/NPC/BP_Enemy.BP_Enemy_C"))
            (bind _arrayelement (Utilities|Array|ReverseforEachLoop _outactors)
              (:LoopBody
                (Utilities|IsValid _arrayelement
                  (:Is%20Valid
                    (Default|MovementTick _arrayelement))))))))
      (else
        (Transformation|SetRelativeLocationAndRotation (Variables|/Game/Core/BP_Character.BP_Character_C|GetSplineMesh (Variables|Default|GetCharacterReference)) (Utilities|Array|Get(acopy) (Variables|Default|GetAttackVector) _output_get) (Utilities|Array|Get(acopy) (Variables|Default|GetAttackRotation) _output_get) false false)))
    (else
      (goto _label))))

(event Custom|AttackEvent
  ;[0.15 0.15 0.15 0.5] SpaceBar
  (if (Variables|Default|GetAttacking?)
    (Default|Attack (Variables|Default|GetCharacterReference))
    (Variables|Default|SetAttacking? false)
    (else
      (Default|Attack (Variables|Default|GetCharacterReference))
      (Variables|Default|SetAttacking? true)))
  (bind _outactors (Actor|GetAllActorsOfClass "/Game/Core/NPC/BP_Enemy.BP_Enemy_C"))
  (bind _arrayelement (Utilities|Array|ReverseforEachLoop _outactors)
    (:LoopBody
      (Utilities|IsValid _arrayelement
        (:Is%20Valid
          (Default|MovementTick _arrayelement))))))

(event Input|EnhancedActionEvents|EnhancedInputActionIA_MoveForward
  (params (ActionValue :type Vector%202D%20Structure) (ElapsedSeconds :type Float%20%28double-precision%29) (TriggeredSeconds :type Float%20%28double-precision%29) (InputAction :type Input%20Action%20Object%20Reference :default "/Game/Core/Interface/Controls/IA_MoveForward.IA_MoveForward"))
  (bind _up_down (Variables|Default|GetUp/Down))
  (bind _left_right (Variables|Default|GetLeft/right))
  (bind _returnvalue (+ _up_down 1.0))
  (bind _returnvalue_2 (+ _left_right 0.0))
  ;[0.15 0.15 0.15 0.5] Movement
  (if (Utilities|Operators|EqualEqual :A (Variables|/Script/Engine.SceneComponent|GetRelativeRotation (Variables|/Game/Core/BP_Character.BP_Character_C|GetSplineMesh (Variables|Default|GetCharacterReference))))
    (Variables|Default|SetChangingAttack? true))
  (if (Variables|/Game/Core/BP_Character.BP_Character_C|GetAttackMarked (Variables|Default|GetCharacterReference))
    (bind _output_get (Variables|Default|SetAttackDirection 0))
    (if (Variables|Default|GetChangingAttack?)
      (Variables|Default|SetChangingAttack? false :!label _label)
      (Default|CancelAttack (Variables|Default|GetCharacterReference) true)
      (bind _valid_ (Utilities|TileValid? _returnvalue _returnvalue_2)
        (:truth%20exe
          (if _valid_
            (CallFunction|MoveCharacter _returnvalue _returnvalue_2)
            (bind _outactors (Actor|GetAllActorsOfClass "/Game/Core/NPC/BP_Enemy.BP_Enemy_C"))
            (bind _arrayelement (Utilities|Array|ReverseforEachLoop _outactors)
              (:LoopBody
                (Utilities|IsValid _arrayelement
                  (:Is%20Valid
                    (Default|MovementTick _arrayelement))))))))
      (else
        (Transformation|SetRelativeLocationAndRotation (Variables|/Game/Core/BP_Character.BP_Character_C|GetSplineMesh (Variables|Default|GetCharacterReference)) (Utilities|Array|Get(acopy) (Variables|Default|GetAttackVector) _output_get) (Utilities|Array|Get(acopy) (Variables|Default|GetAttackRotation) _output_get) false false)))
    (else
      (goto _label))))

(event Input|EnhancedActionEvents|EnhancedInputActionIA_MoveLeft
  (params (ActionValue :type Vector%202D%20Structure) (ElapsedSeconds :type Float%20%28double-precision%29) (TriggeredSeconds :type Float%20%28double-precision%29) (InputAction :type Input%20Action%20Object%20Reference :default "/Game/Core/Interface/Controls/IA_MoveLeft.IA_MoveLeft"))
  (bind _up_down (Variables|Default|GetUp/Down))
  (bind _left_right (Variables|Default|GetLeft/right))
  (bind _returnvalue (+ _up_down 0.0))
  (bind _returnvalue_2 (+ _left_right -1.0))
  ;[0.15 0.15 0.15 0.5] Movement
  (Utilities|Rotate "1.000000,-1.000000,8.000000" "0.000000,-90.000000,90.000000"
    (:NewParam2
      (if (Utilities|Operators|EqualEqual (Variables|/Script/Engine.SceneComponent|GetRelativeRotation (Variables|/Game/Core/BP_Character.BP_Character_C|GetSplineMesh (Variables|Default|GetCharacterReference))) "0.000000,270.000000,0.000000" 0.0)
        (Variables|Default|SetChangingAttack? true))
      (if (Variables|/Game/Core/BP_Character.BP_Character_C|GetAttackMarked (Variables|Default|GetCharacterReference))
        (bind _output_get (Variables|Default|SetAttackDirection 1))
        (if (Variables|Default|GetChangingAttack?)
          (Variables|Default|SetChangingAttack? false :!label _label)
          (Default|CancelAttack (Variables|Default|GetCharacterReference) true)
          (bind _valid_ (Utilities|TileValid? _returnvalue _returnvalue_2)
            (:truth%20exe
              (if _valid_
                (CallFunction|MoveCharacter _returnvalue _returnvalue_2)
                (bind _outactors (Actor|GetAllActorsOfClass "/Game/Core/NPC/BP_Enemy.BP_Enemy_C"))
                (bind _arrayelement (Utilities|Array|ReverseforEachLoop _outactors)
                  (:LoopBody
                    (Utilities|IsValid _arrayelement
                      (:Is%20Valid
                        (Default|MovementTick _arrayelement))))))))
          (else
            (Transformation|SetRelativeLocationAndRotation (Variables|/Game/Core/BP_Character.BP_Character_C|GetSplineMesh (Variables|Default|GetCharacterReference)) (Utilities|Array|Get(acopy) (Variables|Default|GetAttackVector) _output_get) (Utilities|Array|Get(acopy) (Variables|Default|GetAttackRotation) _output_get) false false)))
        (else
          (goto _label))))))

(event Input|EnhancedActionEvents|EnhancedInputActionIA_MoveBack
  (params (ActionValue :type Vector%202D%20Structure) (ElapsedSeconds :type Float%20%28double-precision%29) (TriggeredSeconds :type Float%20%28double-precision%29) (InputAction :type Input%20Action%20Object%20Reference :default "/Game/Core/Interface/Controls/IA_MoveBack.IA_MoveBack"))
  (bind _up_down (Variables|Default|GetUp/Down))
  (bind _left_right (Variables|Default|GetLeft/right))
  (bind _returnvalue (+ _up_down -1.0))
  (bind _returnvalue_2 (+ _left_right 0.0))
  ;[0.15 0.15 0.15 0.5] Movement
  (if (Utilities|Operators|EqualEqual (Variables|/Script/Engine.SceneComponent|GetRelativeRotation (Variables|/Game/Core/BP_Character.BP_Character_C|GetSplineMesh (Variables|Default|GetCharacterReference))) "0.000000,180.000000,0.000000" 0.0)
    (Variables|Default|SetChangingAttack? true))
  (if (Variables|/Game/Core/BP_Character.BP_Character_C|GetAttackMarked (Variables|Default|GetCharacterReference))
    (bind _output_get (Variables|Default|SetAttackDirection 3))
    (if (Variables|Default|GetChangingAttack?)
      (Variables|Default|SetChangingAttack? false :!label _label)
      (Default|CancelAttack (Variables|Default|GetCharacterReference) true)
      (bind _valid_ (Utilities|TileValid? _returnvalue _returnvalue_2)
        (:truth%20exe
          (if _valid_
            (CallFunction|MoveCharacter _returnvalue _returnvalue_2)
            (bind _outactors (Actor|GetAllActorsOfClass "/Game/Core/NPC/BP_Enemy.BP_Enemy_C"))
            (bind _arrayelement (Utilities|Array|ReverseforEachLoop _outactors)
              (:LoopBody
                (Utilities|IsValid _arrayelement
                  (:Is%20Valid
                    (Default|MovementTick _arrayelement))))))))
      (else
        (Transformation|SetRelativeLocationAndRotation (Variables|/Game/Core/BP_Character.BP_Character_C|GetSplineMesh (Variables|Default|GetCharacterReference)) (Utilities|Array|Get(acopy) (Variables|Default|GetAttackVector) _output_get) (Utilities|Array|Get(acopy) (Variables|Default|GetAttackRotation) _output_get) false false)))
    (else
      (goto _label))))

(event Input|EnhancedActionEvents|EnhancedInputActionIA_MoveRight
  (params (ActionValue :type Vector%202D%20Structure) (ElapsedSeconds :type Float%20%28double-precision%29) (TriggeredSeconds :type Float%20%28double-precision%29) (InputAction :type Input%20Action%20Object%20Reference :default "/Game/Core/Interface/Controls/IA_MoveRight.IA_MoveRight"))
  (bind _up_down (Variables|Default|GetUp/Down))
  (bind _left_right (Variables|Default|GetLeft/right))
  (bind _returnvalue (+ _up_down 0.0))
  (bind _returnvalue_2 (+ _left_right 1.0))
  ;[0.15 0.15 0.15 0.5] Movement
  (Utilities|Rotate "1.000000,1.000000,8.000000" "180.000000,-90.000000,90.000000"
    (:NewParam2
      (if (Utilities|Operators|EqualEqual (Variables|/Script/Engine.SceneComponent|GetRelativeRotation (Variables|/Game/Core/BP_Character.BP_Character_C|GetSplineMesh (Variables|Default|GetCharacterReference))) "0.000000,90.000000,0.000000" 0.0)
        (Variables|Default|SetChangingAttack? true))
      (if (Variables|/Game/Core/BP_Character.BP_Character_C|GetAttackMarked (Variables|Default|GetCharacterReference))
        (bind _output_get (Variables|Default|SetAttackDirection 2))
        (if (Variables|Default|GetChangingAttack?)
          (Variables|Default|SetChangingAttack? false :!label _label)
          (Default|CancelAttack (Variables|Default|GetCharacterReference) true)
          (bind _valid_ (Utilities|TileValid? _returnvalue _returnvalue_2)
            (:truth%20exe
              (if _valid_
                (CallFunction|MoveCharacter _returnvalue _returnvalue_2)
                (bind _outactors (Actor|GetAllActorsOfClass "/Game/Core/NPC/BP_Enemy.BP_Enemy_C"))
                (bind _arrayelement (Utilities|Array|ReverseforEachLoop _outactors)
                  (:LoopBody
                    (Utilities|IsValid _arrayelement
                      (:Is%20Valid
                        (Default|MovementTick _arrayelement))))))))
          (else
            (Transformation|SetRelativeLocationAndRotation (Variables|/Game/Core/BP_Character.BP_Character_C|GetSplineMesh (Variables|Default|GetCharacterReference)) (Utilities|Array|Get(acopy) (Variables|Default|GetAttackVector) _output_get) (Utilities|Array|Get(acopy) (Variables|Default|GetAttackRotation) _output_get) false false)))
        (else
          (goto _label))))))

(event EventBeginPlay
  ;[0.15 0.15 0.15 0.5] Gamemode Link
  (Variables|Default|SetbShowMouseCursor false)
  (Input|SetInputModeGameOnly self false)
  (Utilities|FlowControl|Sequence
    (:then_0
      (bind _asbp_gamemode (Utilities|Casting|CastToBP_Gamemode (Game|GetGameMode)))
      (Variables|Default|SetBPM (Variables|/Game/Core/BP_Gamemode.BP_Gamemode_C|GetBPM _asbp_gamemode))
      (Variables|Default|SetTile%20Map (Default|GetTIlemap _asbp_gamemode))
      (bind _asbp_character (Utilities|Casting|CastToBP_Character (Game|GetPlayerCharacter 0)))
      (Variables|Default|SetCharacterReference _asbp_character)
      (Input|AddMappingContext (PlayerController|LocalPlayerSubsystems|GetEnhancedInputLocalPlayerSubsystem (Game|GetPlayerController 0)) (Variables|Default|GetMapping%20Context) 0 "(bIgnoreAllPressedKeysUntilRelease=True,bForceImmediately=False,bNotifyUserSettings=False)"))))

(event Input|KeyboardEvents|SpaceBar
  (params (Key :type Key%20Structure))
  ;[0.15 0.15 0.15 0.5] SpaceBar
  (:Pressed
    (if (Variables|Default|GetAttacking?)
      (Default|Attack (Variables|Default|GetCharacterReference))
      (Variables|Default|SetAttacking? false)
      (else
        (Default|Attack (Variables|Default|GetCharacterReference))
        (Variables|Default|SetAttacking? true)))
    (bind _outactors (Actor|GetAllActorsOfClass "/Game/Core/NPC/BP_Enemy.BP_Enemy_C"))
    (bind _arrayelement (Utilities|Array|ReverseforEachLoop _outactors)
      (:LoopBody
        (Utilities|IsValid _arrayelement
          (:Is%20Valid
            (Default|MovementTick _arrayelement)))))))

(fn ConstructionScript)

(fn MoveCharacter
  (params (UpDown :type Integer) (LeftRight :type Integer))
  (Utilities|FlowControl|Sequence
    (:then_0
      (Variables|Default|SetUp/Down UpDown)
      (Variables|Default|SetLeft/right LeftRight))
    (:then_1
      (bind (_tilex _tiley) (Default|TiletoLocation (Variables|Default|GetTile%20Map) (Variables|Default|GetLeft/right) (Variables|Default|GetUp/Down)))
      (Transformation|SetActorLocation (Game|GetPlayerCharacter 0) (Math|Vector|MakeVector _tilex _tiley 5.0) false false)
      (return))))

(fn AttackMove
  (params (Attack%20Movement%20tiles? :type Integer))
  (bind (_arrayindex _arrayelement) (Utilities|Array|ReverseforEachLoop (Variables|Default|GetAttackRotation))
    (:LoopBody
      (if (Utilities|Operators|EqualEqual _arrayelement (Variables|/Script/Engine.SceneComponent|GetRelativeRotation (Variables|/Game/Core/BP_Character.BP_Character_C|GetSplineMesh (Variables|Default|GetCharacterReference))) 1.0)
        (switch int _arrayindex
          (:0
            (Utilities|FlowControl|DoN (Variables|Default|GetAttackMovementWeapon) :!label _label
              (:Exit
                (bind _valid_ (Utilities|TileValid? (+ (Variables|Default|GetUp/Down) (Variables|Default|GetForward%20or%20Back)) (+ (Variables|Default|GetLeft/right) 0))
                  (:truth%20exe
                    (if _valid_
                      (CallFunction|MoveCharacter (+ (Variables|Default|GetUp/Down) (Variables|Default|GetForward%20or%20Back)) (+ (Variables|Default|GetLeft/right) 0))
                      (goto _label)))))))
          (:1
            (Utilities|FlowControl|DoN (Variables|Default|GetAttackMovementWeapon) :!label _label_2
              (:Exit
                (bind _valid__2 (Utilities|TileValid? (+ (Variables|Default|GetUp/Down) 0) (- (Variables|Default|GetLeft/right) (Variables|Default|GetForward%20or%20Back)))
                  (:truth%20exe
                    (if _valid__2
                      (CallFunction|MoveCharacter (+ (Variables|Default|GetUp/Down) 0) (- (Variables|Default|GetLeft/right) (Variables|Default|GetForward%20or%20Back)))
                      (goto _label_2)))))))
          (:2
            (Utilities|FlowControl|DoN (Variables|Default|GetAttackMovementWeapon) :!label _label_3
              (:Exit
                (bind _valid__3 (Utilities|TileValid? (+ (Variables|Default|GetUp/Down) 0) (+ (Variables|Default|GetLeft/right) (Variables|Default|GetForward%20or%20Back)))
                  (:truth%20exe
                    (if _valid__3
                      (CallFunction|MoveCharacter (+ (Variables|Default|GetUp/Down) 0) (+ (Variables|Default|GetLeft/right) (Variables|Default|GetForward%20or%20Back)))
                      (goto _label_3)))))))
          (:3
            (Utilities|FlowControl|DoN (Variables|Default|GetAttackMovementWeapon) :!label _label_4
              (:Exit
                (bind _valid__4 (Utilities|TileValid? (- (Variables|Default|GetUp/Down) (Variables|Default|GetForward%20or%20Back)) (+ (Variables|Default|GetLeft/right) 0))
                  (:truth%20exe
                    (if _valid__4
                      (CallFunction|MoveCharacter (- (Variables|Default|GetUp/Down) (Variables|Default|GetForward%20or%20Back)) (+ (Variables|Default|GetLeft/right) 0))
                      (goto _label_4))))))))))
    (:Completed
      (return))))