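; BP_ItemDrop is a weapon drop item displayed as a Paper2D sprite.
; On BeginPlay it looks up its RowName in the DB_Weapons data table, stores the row as WeaponData and applies that row's sprite to the PaperSprite.
; A copy of the same lookup sits unconnected in the construction script, so the sprite is set only at runtime.
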(event EventBeginPlay
  (bind _returnvalue (Utilities|GetDataTableRow "/Game/Core/Items/Weapons/DB_Weapons.DB_Weapons" (Variables|Default|GetRow%20Name))
    (:then
      (bind _output_get (Variables|Default|SetWeapon%20Data _returnvalue))
      (Rendering|Components|Sprite|SetSprite (Variables|Default|GetPaperSprite) (.Sprite (Utilities|Struct|BreakS_Weapon _output_get))))))

(fn ConstructionScript)