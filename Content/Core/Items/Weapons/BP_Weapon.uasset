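; Weapon pickup actor for a tile-based Paper2D game, with its visuals driven by a data table.
; The construction script looks up the item's row and sets the weapon sprite and animated flipbook.
; Shortly after BeginPlay, it snaps to a hardcoded tile using the game mode's TileMap.
; Overlap by a BP_Character opens the Weapon_PickUI widget and destroys the actor.
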(event EventBeginPlay
  (Utilities|FlowControl|Delay 0.1)
  (bind _asbp_gamemode (Utilities|Casting|CastToBP_Gamemode (Game|GetGameMode)))
  (Variables|Default|SetTile%20Map (Variables|/Game/Core/BP_Gamemode.BP_Gamemode_C|GetTileMap _asbp_gamemode))
  (bind (_tilex _tiley) (Default|TiletoLocation (Variables|Default|GetTile%20Map) 10 7))
  (Transformation|SetActorLocation (Math|Vector|MakeVector _tilex _tiley 5.0) false false))

(event Collision|EventActorBeginOverlap
  (params (OtherActor :type Actor%20Object%20Reference))
  (bind _asbp_character (Utilities|Casting|CastToBP_Character OtherActor))
  (bind _returnvalue (Game|ConstructObjectfromClass _asbp_character "/Game/Core/Items/Weapons/Weapon_PickUI.Weapon_PickUI_C"))
  (UserInterface|Viewport|AddtoViewport _returnvalue 0)
  (Actor|DestroyActor))

(fn ConstructionScript
  (bind _itemdata (Variables|Default|GetItemData))
  (bind _returnvalue (Utilities|GetDataTableRow (.datatable (.item _itemdata)) (.rowname (.item _itemdata)))
    (:then
      (Rendering|Components|Sprite|SetSprite (Variables|Default|GetWeapon) (.Mesh (Utilities|Struct|BreakS_Weapon _returnvalue)))
      (Sprite|SetFlipbook (Variables|Default|GetAnimatedWeapon) (.AnimatedWeapon (Utilities|Struct|BreakS_Weapon _returnvalue))))))