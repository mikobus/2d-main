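; Weapon chest pickup that opens a weapon selection UI when a character overlaps it.
; On overlap it adds a Weapon_PickUI widget to the viewport, spawns a coin burst effect and destroys itself.
; BeginPlay caches the game mode's TileMap after a short delay, but the tile-based positioning that uses it is disconnected.
; The construction script stops the AnimatedWeapon component.
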(event EventBeginPlay
  (Utilities|FlowControl|Delay 0.1)
  (bind _asbp_gamemode (Utilities|Casting|CastToBP_Gamemode (Game|GetGameMode)))
  (Variables|Default|SetTile%20Map (Variables|/Game/Core/BP_Gamemode.BP_Gamemode_C|GetTileMap _asbp_gamemode)))

(event Collision|EventActorBeginOverlap
  (params (OtherActor :type Actor%20Object%20Reference))
  (bind _asbp_character (Utilities|Casting|CastToBP_Character OtherActor))
  (bind _returnvalue (Game|ConstructObjectfromClass _asbp_character "/Game/Core/Items/Weapons/Weapon_PickUI.Weapon_PickUI_C"))
  (UserInterface|Viewport|AddtoViewport _returnvalue 0)
  (Niagara|SpawnSystematLocation "/Game/Core/assets/Effects/CoinBurst.CoinBurst" (Transformation|GetActorLocation))
  (Actor|DestroyActor))

(fn ConstructionScript
  (Audio|Components|Audio|Stop (Variables|Default|GetAnimatedWeapon)))