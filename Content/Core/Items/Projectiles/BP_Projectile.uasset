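; BP_Projectile is a projectile actor that destroys itself when it hits an enemy or leaves the player's spline mesh.
; On BeginPlay it caches the SplineMesh component from player 0's BP_Character.
; Its Box collision drives both exits: begin overlap with an actor tagged Enemy, or end overlap with that cached mesh.
; The graph itself contains no movement or damage logic.
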(event OnComponentEndOverlap(Box)
  (params (OverlappedComponent :type Primitive%20Component%20Object%20Reference) (OtherActor :type Actor%20Object%20Reference) (OtherComp :type Primitive%20Component%20Object%20Reference) (OtherBodyIndex :type Integer))
  (if (== OtherComp (Variables|Default|GetSpline%20Mesh))
    (Actor|DestroyActor)))

(event OnComponentBeginOverlap(Box)
  (params (OverlappedComponent :type Primitive%20Component%20Object%20Reference) (OtherActor :type Actor%20Object%20Reference) (OtherComp :type Primitive%20Component%20Object%20Reference) (OtherBodyIndex :type Integer) (bFromSweep :type Boolean) (SweepResult :type Hit%20Result%20Structure%20%28by%20ref%29))
  (if (Actor|ActorHasTag OtherActor "Enemy")
    (Actor|DestroyActor)))

(event EventBeginPlay
  (bind _asbp_character (Utilities|Casting|CastToBP_Character (Game|GetPlayerCharacter 0)))
  (Variables|Default|SetSpline%20Mesh (Variables|/Game/Core/BP_Character.BP_Character_C|GetSplineMesh _asbp_character)))

(fn ConstructionScript)