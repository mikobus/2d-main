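; BP_SwordWeapon is a melee sword whose UseWeapon event drives attacks through the player character's SplineMesh and PaperFlipbook.
; The first use sizes the mesh from WeaponData range and width and holds a FullAttack frame as a pose.
; Later uses damage every overlapping BP_Enemy with sparks and sounds, scaled by DamageMult.
; Hits pick stab, downstab or full-attack animation from mesh rotation, while misses play Dodge1.
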(event EventUseWeapon
  (bind _weapondata (Variables|Default|GetWeaponData))
  (bind _weapondata_2 (Variables|Default|GetWeaponData))
  ;[0.15 0.15 0.15 0.5] Melee Attack
  (bind _asbp_character (Utilities|Casting|CastToBP_Character (Game|GetPlayerCharacter 0)))
  (Variables|Default|SetAs%20BP%20Character _asbp_character)
  (if (Variables|Default|GetCondition)
    (Collision|SetCollisionEnabled (Variables|/Game/Core/BP_Character.BP_Character_C|GetSplineMesh (Variables|Default|GetAs%20BP%20Character)) "QueryAndPhysics")
    (if (> (Utilities|Array|Length (Collision|GetOverlappingActors (Variables|/Game/Core/BP_Character.BP_Character_C|GetSplineMesh (Variables|Default|GetAs%20BP%20Character)) "/Game/Core/NPC/BP_Enemy.BP_Enemy_C" :!class /Script/Engine.PrimitiveComponent)) 0)
      (bind _arrayelement (Utilities|Array|ReverseforEachLoop (Collision|GetOverlappingActors (Variables|/Game/Core/BP_Character.BP_Character_C|GetSplineMesh (Variables|Default|GetAs%20BP%20Character)) "/Game/Core/NPC/BP_Enemy.BP_Enemy_C" :!class /Script/Engine.PrimitiveComponent))
        (:LoopBody
          (Niagara|SpawnSystematLocation "/Game/Core/assets/Effects/Sparks.Sparks" (Transformation|GetActorLocation _arrayelement) (Math|Rotator|FindLookatRotation (Transformation|GetActorLocation (Game|GetPlayerCharacter 0)) (Transformation|GetActorLocation _arrayelement)))
          (Game|Damage|ApplyDamage _arrayelement (* (.damage _weapondata_2) (Variables|/Game/Core/BP_Character.BP_Character_C|GetDamageMult (Variables|Default|GetAs%20BP%20Character))) 0 (Variables|Default|GetAs%20BP%20Character) "/Engine/EngineDamageTypes/DmgTypeBP_Environmental.DmgTypeBP_Environmental_C")
          (Audio|PlaySound2D (.hitsound _weapondata_2) 1.0 1.0 0.0 0 0))
        (:Completed
          ;;[0.15 0.15 0.15 0.5] Animations
          (if (Utilities|Operators|EqualEqual :A (Transformation|GetWorldRotation (Variables|/Game/Core/BP_Character.BP_Character_C|GetSplineMesh (Variables|Default|GetAs%20BP%20Character))) :ErrorTolerance 1.0)
            (Sprite|SetFlipbook (Variables|/Game/Core/BP_Character.BP_Character_C|GetPaperFlipbook (Variables|Default|GetAs%20BP%20Character)) "/Game/Core/Spirtes/Human/Melee/StabAttack.StabAttack")
            (elif (Utilities|Operators|EqualEqual (Transformation|GetWorldRotation (Variables|/Game/Core/BP_Character.BP_Character_C|GetSplineMesh (Variables|Default|GetAs%20BP%20Character))) "0.000000,180.000000,0.000000" 1.0)
              (Sprite|SetFlipbook (Variables|/Game/Core/BP_Character.BP_Character_C|GetPaperFlipbook (Variables|Default|GetAs%20BP%20Character)) "/Game/Core/Spirtes/Human/Melee/Downstab.Downstab")
              (else
                (Sprite|SetFlipbook (Variables|/Game/Core/BP_Character.BP_Character_C|GetPaperFlipbook (Variables|Default|GetAs%20BP%20Character)) "/Game/Core/Spirtes/Human/Melee/FullAttack.FullAttack"))))
          (Audio|PlaySound2D (.swingsound (Variables|Default|GetWeaponData)) 1.0 1.0 0.0 0 0)
          (Components|Activation|SetActive (Variables|/Game/Core/BP_Character.BP_Character_C|GetSwingEffect (Variables|Default|GetAs%20BP%20Character)) true false)
          (Components|Timeline|PlayfromStart (Variables|/Game/Core/BP_Character.BP_Character_C|GetPaperFlipbook (Variables|Default|GetAs%20BP%20Character)) :!label _label)
          (Components|Timeline|SetLooping (Variables|/Game/Core/BP_Character.BP_Character_C|GetPaperFlipbook (Variables|Default|GetAs%20BP%20Character)) false)))
      (else
        (Sprite|SetFlipbook (Variables|/Game/Core/BP_Character.BP_Character_C|GetPaperFlipbook (Variables|Default|GetAs%20BP%20Character)) "/Game/Core/Spirtes/Human/Melee/Dodge1.Dodge1")
        (goto _label)))
    (else
      (Variables|Default|SetCondition true)
      (Transformation|SetRelativeTransform (Variables|/Game/Core/BP_Character.BP_Character_C|GetSplineMesh (Variables|Default|GetAs%20BP%20Character)) (Math|Transform|MakeTransform (.location (Transformation|GetRelativeTransform (Variables|/Game/Core/BP_Character.BP_Character_C|GetSplineMesh (Variables|Default|GetAs%20BP%20Character)))) (.rotation (Transformation|GetRelativeTransform (Variables|/Game/Core/BP_Character.BP_Character_C|GetSplineMesh (Variables|Default|GetAs%20BP%20Character)))) (Math|Vector|MakeVector (* (.range _weapondata) 0.32) (* (.width _weapondata) 0.32) 5.0)) false false)
      (Sprite|SetFlipbook (Variables|/Game/Core/BP_Character.BP_Character_C|GetPaperFlipbook (Variables|Default|GetAs%20BP%20Character)) "/Game/Core/Spirtes/Human/Melee/FullAttack.FullAttack")
      (Class|PaperFlipbookComponent|SetPlaybackPositioninFrames (Variables|/Game/Core/BP_Character.BP_Character_C|GetPaperFlipbook (Variables|Default|GetAs%20BP%20Character)) 2 false)
      (Audio|Components|Audio|Stop (Variables|/Game/Core/BP_Character.BP_Character_C|GetPaperFlipbook (Variables|Default|GetAs%20BP%20Character))))))

(fn ConstructionScript)