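; Bow weapon for the player character that fires piercing ranged attacks at enemies.
; UseWeapon sizes the character's SplineMesh by weapon range and width to gather overlapping BP_Enemy actors, reverting to the idle flipbook when none are found.
; With targets, it plays the throw animation and spawns an arrow along the aim direction.
; Damage applies directly through a DoN loop over the nearest targets, bounded by PierceCount and scaled by DamageMult, with sparks and sounds.
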(event EventUseWeapon
  (bind _weapondata (Variables|Default|GetWeaponData))
  (bind _weapondata_2 (Variables|Default|GetWeaponData))
  (bind _weapondata_3 (Variables|Default|GetWeaponData))
  ;[0.15 0.15 0.15 0.5] RangedAttack
  (bind _asbp_character (Utilities|Casting|CastToBP_Character (Game|GetPlayerCharacter 0)))
  (Variables|Default|SetAs%20BP%20Character _asbp_character)
  (Transformation|SetRelativeTransform (Variables|/Game/Core/BP_Character.BP_Character_C|GetSplineMesh (Variables|Default|GetAs%20BP%20Character)) (Math|Transform|MakeTransform (.location (Transformation|GetRelativeTransform (Variables|/Game/Core/BP_Character.BP_Character_C|GetSplineMesh (Variables|Default|GetAs%20BP%20Character)))) (.rotation (Transformation|GetRelativeTransform (Variables|/Game/Core/BP_Character.BP_Character_C|GetSplineMesh (Variables|Default|GetAs%20BP%20Character)))) (Math|Vector|MakeVector (* (.range _weapondata_2) 0.32) (* (.width _weapondata_2) 0.32) 5.0)) false false)
  (Collision|SetCollisionEnabled (Variables|/Game/Core/BP_Character.BP_Character_C|GetSplineMesh (Variables|Default|GetAs%20BP%20Character)) "QueryAndPhysics")
  (bind _output_get (Variables|Default|SetOverlapping%20Actors (Collision|GetOverlappingActors (Variables|/Game/Core/BP_Character.BP_Character_C|GetSplineMesh (Variables|Default|GetAs%20BP%20Character)) "/Game/Core/NPC/BP_Enemy.BP_Enemy_C" :!class /Script/Engine.PrimitiveComponent)))
  (if (> (Utilities|Array|Length _output_get) 0)
    (Sprite|SetFlipbook (Variables|/Game/Core/BP_Character.BP_Character_C|GetPaperFlipbook (Variables|Default|GetAs%20BP%20Character)) "/Game/Core/Spirtes/Human/Melee/TrollThrow.TrollThrow")
    (Components|Timeline|PlayfromStart (Variables|/Game/Core/BP_Character.BP_Character_C|GetPaperFlipbook (Variables|Default|GetAs%20BP%20Character)))
    (Components|Timeline|SetLooping (Variables|/Game/Core/BP_Character.BP_Character_C|GetPaperFlipbook (Variables|Default|GetAs%20BP%20Character)) false)
    (Audio|PlaySound2D (.swingsound _weapondata_3) 1.0 1.0 0.0 0 0)
    (Game|SpawnActorfromClass "/Game/Core/Items/Projectiles/BP_Arrow1.BP_Arrow1_C" (Math|Transform|MakeTransform (.location (Transformation|GetWorldTransform (Variables|/Game/Core/BP_Character.BP_Character_C|GetAimingDirection (Variables|Default|GetAs%20BP%20Character)))) (.rotation (Transformation|GetWorldTransform (Variables|/Game/Core/BP_Character.BP_Character_C|GetAimingDirection (Variables|Default|GetAs%20BP%20Character)))) "1.000000,1.000000,1.000000") "Undefined" "MultiplyWithRoot" 0 0)
    (Rendering|SetVisibility (Variables|/Game/Core/BP_Character.BP_Character_C|GetArrows (Variables|Default|GetAs%20BP%20Character)) false false)
    (bind _counter (Utilities|FlowControl|DoN (.piercecount _weapondata_3) :!label _label)
      (:Exit
        (Rendering|SetVisibility (Variables|Default|GetPaperSprite) false false)
        (if (Utilities|IsValid (.ReturnValue (Actor|FindNearestActor (Transformation|GetActorLocation (Variables|Default|GetAs%20BP%20Character)) (Variables|Default|GetOverlapping%20Actors))))
          (Niagara|SpawnSystematLocation "/Game/Core/assets/Effects/Sparks.Sparks" (Transformation|GetActorLocation (.ReturnValue (Actor|FindNearestActor (Transformation|GetActorLocation (Variables|Default|GetAs%20BP%20Character)) (Variables|Default|GetOverlapping%20Actors)))) (Math|Rotator|FindLookatRotation (Transformation|GetActorLocation (Variables|Default|GetAs%20BP%20Character)) (Transformation|GetActorLocation (.ReturnValue (Actor|FindNearestActor (Transformation|GetActorLocation (Variables|Default|GetAs%20BP%20Character)) (Variables|Default|GetOverlapping%20Actors)))))))
        (Game|Damage|ApplyDamage (.ReturnValue (Actor|FindNearestActor (Transformation|GetActorLocation (Variables|Default|GetAs%20BP%20Character)) (Variables|Default|GetOverlapping%20Actors))) (* (.damage _weapondata) (Variables|/Game/Core/BP_Character.BP_Character_C|GetDamageMult (Variables|Default|GetAs%20BP%20Character))) 0 0)
        (Utilities|Array|RemoveItem (Variables|Default|GetOverlapping%20Actors) (.ReturnValue (Actor|FindNearestActor (Transformation|GetActorLocation (Variables|Default|GetAs%20BP%20Character)) (Variables|Default|GetOverlapping%20Actors))))
        (Audio|PlaySound2D (.hitsound _weapondata) 1.0 1.0 0.0 0 0)
        (if (== _counter (.piercecount _weapondata))
          (goto _label Reset)
          (else
            (goto _label)))))
    (else
      (Sprite|SetFlipbook (Variables|/Game/Core/BP_Character.BP_Character_C|GetPaperFlipbook (Variables|Default|GetAs%20BP%20Character)) "/Game/Core/Spirtes/Human/Melee/TrollMeleeIdleFB.TrollMeleeIdleFB")
      (Audio|Components|Audio|Play (Variables|/Game/Core/BP_Character.BP_Character_C|GetPaperFlipbook (Variables|Default|GetAs%20BP%20Character)))
      (Components|Timeline|SetLooping (Variables|/Game/Core/BP_Character.BP_Character_C|GetPaperFlipbook (Variables|Default|GetAs%20BP%20Character)) true)
      (Rendering|SetVisibility (Variables|Default|GetPaperSprite) true false)
      (goto _label Reset))))

(fn ConstructionScript
  (|CallParentFunction))