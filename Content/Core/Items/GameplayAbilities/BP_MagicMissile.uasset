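; Magic Missile weapon ability that fires spell projectiles for the player in a tile-based 2D game.
; An initial UseWeapon call shows the character's SplineMesh as an aiming area sized from weapon range and width.
; A later call spawns one projectile per overlapped enemy at the tile-snapped aim point, with directional attack flipbook, sound and effect.
; Without targets it plays a dodge flipbook; NPC use only stores the reference.
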(event EventUseWeapon
  (params (NPC%20Using? :type Boolean) (NPC :type BP%20Enemy%20Object%20Reference))
  (bind _weapondata (Variables|Default|GetWeaponData))
  (if (not NPC%20Using?)
    (bind _asbp_character (Utilities|Casting|CastToBP_Character (Game|GetPlayerCharacter 0)))
    (Variables|Default|SetController%20Ref (Variables|/Game/Core/BP_Character.BP_Character_C|GetControllerRef _asbp_character))
    (Variables|Default|SetAs%20BP%20Character _asbp_character)
    (if (Variables|Default|GetCondition)
      (Variables|Default|SetCondition true)
      (Collision|SetCollisionEnabled (Variables|/Game/Core/BP_Character.BP_Character_C|GetSplineMesh (Variables|Default|GetAs%20BP%20Character)) "QueryAndPhysics")
      (if (> (Utilities|Array|Length (Collision|GetOverlappingActors (Variables|/Game/Core/BP_Character.BP_Character_C|GetSplineMesh (Variables|Default|GetAs%20BP%20Character)) "/Game/Core/NPC/BP_Enemy.BP_Enemy_C" :!class /Script/Engine.PrimitiveComponent)) 0)
        (Utilities|Array|ReverseforEachLoop (Collision|GetOverlappingActors (Variables|/Game/Core/BP_Character.BP_Character_C|GetSplineMesh (Variables|Default|GetAs%20BP%20Character)) "/Game/Core/NPC/BP_Enemy.BP_Enemy_C" :!class /Script/Engine.PrimitiveComponent)
          (:LoopBody
            (bind (_updown _leftright) (Default|LocationtoTile (Variables|/Game/Core/BP_Character.BP_Character_C|GetTile%20Map (Variables|Default|GetAs%20BP%20Character)) (Transformation|GetWorldLocation (Variables|/Game/Core/BP_Character.BP_Character_C|GetAimingDirection (Variables|Default|GetAs%20BP%20Character)))))
            (bind (_tilex _tiley) (Default|TiletoLocation (Variables|/Game/Core/BP_Character.BP_Character_C|GetTile%20Map (Variables|Default|GetAs%20BP%20Character)) _leftright _updown))
            (Game|SpawnActorfromClass "/Game/Core/Items/GameplayAbilities/Projectiles/Spell_Projectile.Spell_Projectile_C" (Math|Transform|MakeTransform (Math|Vector|MakeVector _tilex _tiley 0.0) "0, 0, 0" "1.000000,1.000000,1.000000") "Undefined" "MultiplyWithRoot" 0 (Variables|Default|GetAs%20BP%20Character) (Variables|/Game/Core/BP_Controller.BP_Controller_C|GetAttackDirection (Variables|Default|GetController%20Ref)) (.Damage (Utilities|Struct|BreakS_Weapon (Variables|Default|GetWeaponData))) 0))
          (:Completed
            ;[0.15 0.15 0.15 0.5] Animations
            (if (Utilities|Operators|EqualEqual :A (Transformation|GetWorldRotation (Variables|/Game/Core/BP_Character.BP_Character_C|GetSplineMesh (Variables|Default|GetAs%20BP%20Character))) :ErrorTolerance 1.0)
              (Sprite|SetFlipbook (Variables|/Game/Core/BP_Character.BP_Character_C|GetPaperFlipbook (Variables|Default|GetAs%20BP%20Character)) "/Game/Core/Spirtes/Human/Melee/TrolllUPattack.TrolllUPattack")
              (elif (Utilities|Operators|EqualEqual (Transformation|GetWorldRotation (Variables|/Game/Core/BP_Character.BP_Character_C|GetSplineMesh (Variables|Default|GetAs%20BP%20Character))) "0.000000,180.000000,0.000000" 1.0)
                (Sprite|SetFlipbook (Variables|/Game/Core/BP_Character.BP_Character_C|GetPaperFlipbook (Variables|Default|GetAs%20BP%20Character)) "/Game/Core/Spirtes/Human/Melee/TrollDownSw1.TrollDownSw1")
                (else
                  (Sprite|SetFlipbook (Variables|/Game/Core/BP_Character.BP_Character_C|GetPaperFlipbook (Variables|Default|GetAs%20BP%20Character)) "/Game/Core/Spirtes/Human/Melee/TrollSwing.TrollSwing"))))
            (Audio|PlaySound2D (.swingsound (Variables|Default|GetWeaponData)) 1.0 1.0 0.0 0 0)
            (Components|Activation|SetActive (Variables|/Game/Core/BP_Character.BP_Character_C|GetSwingEffect (Variables|Default|GetAs%20BP%20Character)) true false)
            (Components|Timeline|PlayfromStart (Variables|/Game/Core/BP_Character.BP_Character_C|GetPaperFlipbook (Variables|Default|GetAs%20BP%20Character)))
            (Components|Timeline|SetLooping (Variables|/Game/Core/BP_Character.BP_Character_C|GetPaperFlipbook (Variables|Default|GetAs%20BP%20Character)) false)))
        (else
          (Sprite|SetFlipbook (Variables|/Game/Core/BP_Character.BP_Character_C|GetPaperFlipbook (Variables|Default|GetAs%20BP%20Character)) "/Game/Core/Spirtes/Human/Melee/TrollDodge1.TrollDodge1")
          (Components|Activation|SetActive (Variables|/Game/Core/BP_Character.BP_Character_C|GetSwingEffect (Variables|Default|GetAs%20BP%20Character)) false false)))
      (else
        (Variables|Default|SetCondition true)
        (Rendering|SetVisibility (Variables|/Game/Core/BP_Character.BP_Character_C|GetSplineMesh (Variables|Default|GetAs%20BP%20Character)) true false)
        (Transformation|SetRelativeTransform (Variables|/Game/Core/BP_Character.BP_Character_C|GetSplineMesh (Variables|Default|GetAs%20BP%20Character)) (Math|Transform|MakeTransform (.location (Transformation|GetRelativeTransform (Variables|/Game/Core/BP_Character.BP_Character_C|GetSplineMesh (Variables|Default|GetAs%20BP%20Character)))) (.rotation (Transformation|GetRelativeTransform (Variables|/Game/Core/BP_Character.BP_Character_C|GetSplineMesh (Variables|Default|GetAs%20BP%20Character)))) (Math|Vector|MakeVector (* (.range _weapondata) 0.32) (* (.width _weapondata) 0.32) 5.0)) false false)))
    (else
      (Variables|Default|SetNPC NPC))))

(fn ConstructionScript
  (|CallParentFunction))