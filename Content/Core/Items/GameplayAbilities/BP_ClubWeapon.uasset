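; Club melee weapon whose UseWeapon event serves both the player and NPCs in a Paper2D flipbook game.
; The first use shows a SplineMesh hit area sized from WeaponData and holds a wind-up frame.
; The next damages overlapping enemies, or the player for NPCs, scaled by Strength, with sparks, sounds and rotation-based attack flipbooks.
; NPC strikes reset that state; the player's reset is unwired, and player misses play a dodge.
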(event EventUseWeapon
  (params (NPC%20Using? :type Boolean) (NPC :type BP%20Enemy%20Object%20Reference))
  (bind _returnvalue (Game|GetPlayerCharacter 0))
  (bind _as_bp_character (Variables|Default|GetAs%20BP%20Character))
  (bind _as_bp_character_2 (Variables|Default|GetAs%20BP%20Character))
  (bind _weapondata (Variables|Default|GetWeaponData))
  (bind _as_bp_character_3 (Variables|Default|GetAs%20BP%20Character))
  (bind _as_bp_character_4 (Variables|Default|GetAs%20BP%20Character))
  (bind _weapondata_2 (Variables|Default|GetWeaponData))
  (bind _as_bp_character_5 (Variables|Default|GetAs%20BP%20Character))
  (bind _as_bp_character_6 (Variables|Default|GetAs%20BP%20Character))
  (bind _returnvalue_2 (Transformation|GetActorLocation _returnvalue))
  (bind _splinemesh (Variables|/Game/Core/BP_Character.BP_Character_C|GetSplineMesh _as_bp_character))
  (bind _paperflipbook (Variables|/Game/Core/BP_Character.BP_Character_C|GetPaperFlipbook _as_bp_character_2))
  (bind _splinemesh_2 (Variables|/Game/Core/BP_Character.BP_Character_C|GetSplineMesh _as_bp_character_3))
  (bind _paperflipbook_2 (Variables|/Game/Core/BP_Character.BP_Character_C|GetPaperFlipbook _as_bp_character_4))
  (bind _paperflipbook_3 (Variables|/Game/Core/BP_Character.BP_Character_C|GetPaperFlipbook _as_bp_character_5))
  (bind _returnvalue_3 (Transformation|GetRelativeTransform _splinemesh))
  (bind _overlappingactors (Collision|GetOverlappingActors _splinemesh_2 "/Game/Core/NPC/BP_Enemy.BP_Enemy_C" :!class /Script/Engine.PrimitiveComponent))
  ;[0.15 0.15 0.15 0.5] Melee Attack
  (if (not NPC%20Using?)
    (if (Variables|Default|GetCondition)
      (Collision|SetCollisionEnabled (Variables|/Game/Core/BP_Character.BP_Character_C|GetSplineMesh (Variables|Default|GetAs%20BP%20Character)) "QueryAndPhysics")
      (if (> (Utilities|Array|Length _overlappingactors) 0)
        (bind _arrayelement (Utilities|Array|ReverseforEachLoop _overlappingactors)
          (:LoopBody
            (Niagara|SpawnSystematLocation "/Game/Core/assets/Effects/Sparks.Sparks" (Transformation|GetActorLocation _arrayelement) (Math|Rotator|FindLookatRotation (Transformation|GetActorLocation (Game|GetPlayerCharacter 0)) (Transformation|GetActorLocation _arrayelement)))
            (bind _returnvalue_4 (Game|Damage|ApplyDamage _arrayelement (* (.damage (Variables|Default|GetWeaponData)) (Variables|/Game/Core/Inventory.Inventory_C|GetStrength (Variables|/Game/Core/BP_Character.BP_Character_C|GetInventory _as_bp_character_6))) 0 _as_bp_character_6 "/Engine/EngineDamageTypes/DmgTypeBP_Environmental.DmgTypeBP_Environmental_C"))
            (CallFunction|DPS _returnvalue_4)
            (Audio|PlaySound2D (.HitSound (Utilities|Struct|BreakS_Weapon (Variables|Default|GetWeaponData))) 1.0 1.0 0.0 0 0))
          (:Completed
            ;;[0.15 0.15 0.15 0.5] Animations
            (if (Utilities|Operators|EqualEqual :A (Transformation|GetWorldRotation (Variables|/Game/Core/BP_Character.BP_Character_C|GetSplineMesh (Variables|Default|GetAs%20BP%20Character))) :ErrorTolerance 1.0)
              (Sprite|SetFlipbook _paperflipbook_2 "/Game/Core/Spirtes/Human/Melee/TrolllUPattack.TrolllUPattack")
              (elif (Utilities|Operators|EqualEqual (Transformation|GetWorldRotation (Variables|/Game/Core/BP_Character.BP_Character_C|GetSplineMesh (Variables|Default|GetAs%20BP%20Character))) "0.000000,180.000000,0.000000" 1.0)
                (Sprite|SetFlipbook _paperflipbook_2 "/Game/Core/Spirtes/Human/Melee/TrollDownSw1.TrollDownSw1")
                (else
                  (Sprite|SetFlipbook _paperflipbook_2 "/Game/Core/Spirtes/Human/Melee/TrollSwing.TrollSwing"))))
            (Audio|PlaySound2D (.swingsound (Variables|Default|GetWeaponData)) 1.0 1.0 0.0 0 0)
            (Components|Activation|SetActive (Variables|/Game/Core/BP_Character.BP_Character_C|GetSwingEffect (Variables|Default|GetAs%20BP%20Character)) true false)
            (Components|Timeline|PlayfromStart _paperflipbook_3 :!label _label)
            (Components|Timeline|SetLooping _paperflipbook_3 false)))
        (else
          (Sprite|SetFlipbook _paperflipbook_2 "/Game/Core/Spirtes/Human/Melee/TrollDodge1.TrollDodge1")
          (Components|Activation|SetActive (Variables|/Game/Core/BP_Character.BP_Character_C|GetSwingEffect (Variables|Default|GetAs%20BP%20Character)) false false)
          (goto _label)))
      (else
        (Variables|Default|SetCondition true)
        (Transformation|SetRelativeTransform _splinemesh (Math|Transform|MakeTransform (.location _returnvalue_3) (.rotation _returnvalue_3) (Math|Vector|MakeVector (* (.range _weapondata) 0.32) (* (.width _weapondata) 0.32) 5.0)) false false)
        (Sprite|SetFlipbook (Variables|/Game/Core/BP_Character.BP_Character_C|GetPaperFlipbook (Variables|Default|GetAs%20BP%20Character)) "/Game/Core/Spirtes/Human/Melee/TrollSwing.TrollSwing")
        (Class|PaperFlipbookComponent|SetPlaybackPositioninFrames _paperflipbook 2 false)
        (Audio|Components|Audio|Stop _paperflipbook)
        (Rendering|SetVisibility (Variables|/Game/Core/BP_Character.BP_Character_C|GetSplineMesh _as_bp_character_2) true false)))
    (else
      (Variables|Default|SetNPC NPC)
      (if (Variables|Default|GetCondition)
        (Collision|SetCollisionEnabled (Variables|/Game/Core/NPC/BP_Enemy.BP_Enemy_C|GetSplineMesh (Variables|Default|GetNPC)) "QueryAndPhysics")
        (if (Class|PrimitiveComponent|IsOverlappingComponent (Variables|/Game/Core/NPC/BP_Enemy.BP_Enemy_C|GetSplineMesh (Variables|Default|GetNPC)) (Variables|/Script/Engine.Character|GetCapsuleComponent (Game|GetPlayerCharacter 0)))
          (Utilities|FlowControl|Sequence
            (:then_0
              (Niagara|SpawnSystematLocation "/Game/Core/assets/Effects/Sparks.Sparks" _returnvalue_2 (Math|Rotator|FindLookatRotation (Transformation|GetActorLocation) _returnvalue_2))
              (bind _returnvalue_5 (Game|Damage|ApplyDamage _returnvalue (* (.damage (Variables|Default|GetWeaponData)) (Variables|/Game/Core/Inventory.Inventory_C|GetStrength (Variables|/Game/Core/NPC/BP_Enemy.BP_Enemy_C|GetInventory (Variables|Default|GetNPC)))) 0 (Variables|Default|GetNPC) "/Engine/EngineDamageTypes/DmgTypeBP_Environmental.DmgTypeBP_Environmental_C"))
              (CallFunction|DPS _returnvalue_5)
              (Audio|PlaySound2D (.HitSound (Utilities|Struct|BreakS_Weapon (Variables|Default|GetWeaponData))) 1.0 1.0 0.0 0 0)
              (Variables|Default|SetPlayerHit? true))
            (:then_1
              ;[0.15 0.15 0.15 0.5] Animations
              (if (Utilities|Operators|EqualEqual :A (Transformation|GetWorldRotation (Variables|/Game/Core/NPC/BP_Enemy.BP_Enemy_C|GetSplineMesh (Variables|Default|GetNPC))) :ErrorTolerance 1.0) :!label _label_2
                (Sprite|SetFlipbook (Variables|/Game/Core/NPC/BP_Enemy.BP_Enemy_C|GetPaperFlipbook (Variables|Default|GetNPC)) "/Game/Core/Spirtes/Human/Melee/StabAttack.StabAttack")
                (elif (Utilities|Operators|EqualEqual (Transformation|GetWorldRotation (Variables|/Game/Core/NPC/BP_Enemy.BP_Enemy_C|GetSplineMesh (Variables|Default|GetNPC))) "0.000000,180.000000,0.000000" 1.0)
                  (Sprite|SetFlipbook (Variables|/Game/Core/NPC/BP_Enemy.BP_Enemy_C|GetPaperFlipbook (Variables|Default|GetNPC)) "/Game/Core/Spirtes/Human/Melee/Downstab.Downstab")
                  (else
                    (Sprite|SetFlipbook (Variables|/Game/Core/NPC/BP_Enemy.BP_Enemy_C|GetPaperFlipbook (Variables|Default|GetNPC)) "/Game/Core/Spirtes/Human/Melee/FullAttack.FullAttack"))))
              (Audio|PlaySound2D (.SwingSound (Utilities|Struct|BreakS_Weapon (Variables|Default|GetWeaponData))) 1.0 1.0 0.0 0 0)
              (Components|Timeline|PlayfromStart (Variables|/Game/Core/NPC/BP_Enemy.BP_Enemy_C|GetPaperFlipbook (Variables|Default|GetNPC)))
              (Components|Timeline|SetLooping (Variables|/Game/Core/NPC/BP_Enemy.BP_Enemy_C|GetPaperFlipbook (Variables|Default|GetNPC)) false)
              (Variables|Default|SetCondition false)
              (Rendering|SetVisibility (Variables|/Game/Core/NPC/BP_Enemy.BP_Enemy_C|GetSplineMesh (Variables|Default|GetNPC)) false false)))
          (else
            (Variables|Default|SetPlayerHit? false)
            (goto _label_2)))
        (else
          (Variables|Default|SetCondition true)
          (Transformation|SetRelativeTransform (Variables|/Game/Core/NPC/BP_Enemy.BP_Enemy_C|GetSplineMesh (Variables|Default|GetNPC)) (Math|Transform|MakeTransform (.location (Transformation|GetRelativeTransform (Variables|/Game/Core/NPC/BP_Enemy.BP_Enemy_C|GetSplineMesh (Variables|Default|GetNPC)))) (.rotation (Transformation|GetRelativeTransform (Variables|/Game/Core/NPC/BP_Enemy.BP_Enemy_C|GetSplineMesh (Variables|Default|GetNPC)))) (Math|Vector|MakeVector (* (.range _weapondata_2) 0.32) (* (.width _weapondata_2) 0.32) 5.0)) false false)
          (Sprite|SetFlipbook (Variables|/Game/Core/NPC/BP_Enemy.BP_Enemy_C|GetPaperFlipbook (Variables|Default|GetNPC)) (Variables|/Game/Core/NPC/BP_Enemy.BP_Enemy_C|GetAttack%20Animation (Variables|Default|GetNPC)))
          (Class|PaperFlipbookComponent|SetPlaybackPositioninFrames (Variables|/Game/Core/NPC/BP_Enemy.BP_Enemy_C|GetPaperFlipbook (Variables|Default|GetNPC)) 2 false)
          (Audio|Components|Audio|Stop (Variables|/Game/Core/NPC/BP_Enemy.BP_Enemy_C|GetPaperFlipbook (Variables|Default|GetNPC)))
          (Rendering|SetVisibility (Variables|/Game/Core/NPC/BP_Enemy.BP_Enemy_C|GetSplineMesh (Variables|Default|GetNPC)) true false))))))

(fn ConstructionScript)