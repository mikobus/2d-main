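; BP_Staff is a melee staff weapon that both the player and NPCs attack with through UseWeapon.
; The first call scales and shows the user's SplineMesh as a range-and-width hit area and holds a wind-up flipbook frame.
; Later calls deal Strength-scaled damage with sparks to overlapping enemies or player characters, then animate the strike.
; The player branch also plays sounds and disables input, while the NPC branch re-hides the hit area.
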(event Custom|PlayFlipbookRPC
  (bind _npc (Variables|Default|GetNPC))
  (Components|Timeline|PlayfromStart (Variables|/Game/Core/NPC/BP_Enemy.BP_Enemy_C|GetPaperFlipbook _npc))
  (Components|Timeline|SetLooping (Variables|/Game/Core/NPC/BP_Enemy.BP_Enemy_C|GetPaperFlipbook _npc) false))

(event Custom|StopFlipbookRPC
  (Class|PaperFlipbookComponent|SetPlaybackPositioninFrames (Variables|/Game/Core/NPC/BP_Enemy.BP_Enemy_C|GetPaperFlipbook (Variables|Default|GetNPC)) 2 false)
  (Audio|Components|Audio|Stop (Variables|/Game/Core/NPC/BP_Enemy.BP_Enemy_C|GetPaperFlipbook (Variables|Default|GetNPC))))

(event EventUseWeapon
  (params (NPC%20Using? :type Boolean) (NPC :type BP%20Enemy%20Object%20Reference) (Player :type BP%20Character%20Object%20Reference))
  (bind _weapondata (Variables|Default|GetWeaponData))
  (bind _weapondata_2 (Variables|Default|GetWeaponData))
  (if (Variables|Default|GetInUse)
    ;[0.15 0.15 0.15 0.5] Melee Attack
    (if (not NPC%20Using?)
      (Variables|Default|SetAs%20Bp%20Character Player)
      (if (Variables|Default|GetCondition)
        (Collision|SetCollisionEnabled (Variables|/Game/Core/BP_Character.BP_Character_C|GetSplineMesh (Variables|Default|GetAs%20Bp%20Character)) "QueryAndPhysics")
        (if (> (Utilities|Array|Length (Collision|GetOverlappingActors (Variables|/Game/Core/BP_Character.BP_Character_C|GetSplineMesh (Variables|Default|GetAs%20Bp%20Character)) "/Game/Core/NPC/BP_Enemy.BP_Enemy_C" :!class /Script/Engine.PrimitiveComponent)) 0)
          (bind _arrayelement (Utilities|Array|ReverseforEachLoop (Collision|GetOverlappingActors (Variables|/Game/Core/BP_Character.BP_Character_C|GetSplineMesh (Variables|Default|GetAs%20Bp%20Character)) "/Game/Core/NPC/BP_Enemy.BP_Enemy_C" :!class /Script/Engine.PrimitiveComponent))
            (:LoopBody
              (Niagara|SpawnSystematLocation "/Game/Core/assets/Effects/Sparks.Sparks" (Transformation|GetActorLocation _arrayelement) (Math|Rotator|FindLookatRotation (Transformation|GetActorLocation (Game|GetPlayerCharacter 0)) (Transformation|GetActorLocation _arrayelement)))
              (Game|Damage|ApplyDamage _arrayelement (* (.damage (Variables|Default|GetWeaponData)) (Variables|/Game/Core/Inventory.Inventory_C|GetStrength (Variables|/Game/Core/BP_Character.BP_Character_C|GetInventory (Variables|Default|GetAs%20Bp%20Character)))) 0 (Variables|Default|GetAs%20Bp%20Character) "/Engine/EngineDamageTypes/DmgTypeBP_Environmental.DmgTypeBP_Environmental_C")
              (Audio|PlaySound2D (.HitSound (Utilities|Struct|BreakS_Weapon (Variables|Default|GetWeaponData))) 1.0 1.0 0.0 0 0))
            (:Completed
              ;;[0.15 0.15 0.15 0.5] Animations
              (if (Utilities|Operators|EqualEqual :A (Transformation|GetWorldRotation (Variables|/Game/Core/BP_Character.BP_Character_C|GetSplineMesh (Variables|Default|GetAs%20Bp%20Character))) :ErrorTolerance 1.0) :!label _label
                (Default|ChangeAnimation (Variables|Default|GetAs%20Bp%20Character) "NewEnumerator5")
                (elif (Utilities|Operators|EqualEqual (Transformation|GetWorldRotation (Variables|/Game/Core/BP_Character.BP_Character_C|GetSplineMesh (Variables|Default|GetAs%20Bp%20Character))) "0.000000,180.000000,0.000000" 1.0)
                  (Default|ChangeAnimation (Variables|Default|GetAs%20Bp%20Character) "NewEnumerator4")
                  (else
                    (Default|ChangeAnimation (Variables|Default|GetAs%20Bp%20Character) "NewEnumerator3"))))
              (Audio|PlaySound2D (.swingsound (Variables|Default|GetWeaponData)) 1.0 1.0 0.0 0 0)
              (Components|Activation|SetActive (Variables|/Game/Core/BP_Character.BP_Character_C|GetSwingEffect (Variables|Default|GetAs%20Bp%20Character)) true false)
              (bind _asbp_controller (Utilities|Casting|CastToBP_Controller (Pawn|GetController (Variables|Default|GetAs%20Bp%20Character))))
              (Default|DisableInput _asbp_controller)))
          (else
            (goto _label)))
        (else
          (Variables|Default|SetCondition true)
          (Transformation|SetRelativeTransform (Variables|/Game/Core/BP_Character.BP_Character_C|GetSplineMesh (Variables|Default|GetAs%20Bp%20Character)) (Math|Transform|MakeTransform (.location (Transformation|GetRelativeTransform (Variables|/Game/Core/BP_Character.BP_Character_C|GetSplineMesh (Variables|Default|GetAs%20Bp%20Character)))) (.rotation (Transformation|GetRelativeTransform (Variables|/Game/Core/BP_Character.BP_Character_C|GetSplineMesh (Variables|Default|GetAs%20Bp%20Character)))) (Math|Vector|MakeVector (* (.range _weapondata) -0.32) (* (.width _weapondata) -0.32) 5.0)) false false)
          (Sprite|SetFlipbook (Variables|/Game/Core/BP_Character.BP_Character_C|GetPaperFlipbook (Variables|Default|GetAs%20Bp%20Character)) "/Game/Core/Spirtes/Human/Melee/TrollSwing.TrollSwing")
          (Class|PaperFlipbookComponent|SetPlaybackPositioninFrames (Variables|/Game/Core/BP_Character.BP_Character_C|GetPaperFlipbook (Variables|Default|GetAs%20Bp%20Character)) 2 false)
          (Audio|Components|Audio|Stop (Variables|/Game/Core/BP_Character.BP_Character_C|GetPaperFlipbook (Variables|Default|GetAs%20Bp%20Character)))
          (Rendering|SetVisibility (Variables|/Game/Core/BP_Character.BP_Character_C|GetSplineMesh (Variables|Default|GetAs%20Bp%20Character)) true false)))
      (else
        (Variables|Default|SetNPC NPC)
        (if (Variables|Default|GetCondition)
          (Collision|SetCollisionEnabled (Variables|/Game/Core/NPC/BP_Enemy.BP_Enemy_C|GetSplineMesh (Variables|Default|GetNPC)) "QueryAndPhysics")
          (bind _outactors (Actor|GetAllActorsOfClass "/Game/Core/BP_Character.BP_Character_C"))
          (for _array_element _outactors
            (if (Class|PrimitiveComponent|IsOverlappingComponent (Variables|/Game/Core/NPC/BP_Enemy.BP_Enemy_C|GetSplineMesh (Variables|Default|GetNPC)) (Variables|/Script/Engine.Character|GetCapsuleComponent _array_element))
              (Utilities|FlowControl|Sequence
                (:then_0
                  (Niagara|SpawnSystematLocation "/Game/Core/assets/Effects/Sparks2.Sparks2" (Transformation|GetActorLocation _array_element) (Math|Rotator|FindLookatRotation (Transformation|GetActorLocation) (Transformation|GetActorLocation _array_element)))
                  (Game|Damage|ApplyDamage _array_element (* (.damage (Variables|Default|GetWeaponData)) (Variables|/Game/Core/Inventory.Inventory_C|GetStrength (Variables|/Game/Core/NPC/BP_Enemy.BP_Enemy_C|GetInventory (Variables|Default|GetNPC)))) 0 (Variables|Default|GetNPC) "/Engine/EngineDamageTypes/DmgTypeBP_Environmental.DmgTypeBP_Environmental_C")
                  (Variables|Default|SetPlayerHit? true))
                (:then_1
                  ;[0.15 0.15 0.15 0.5] Animations
                  (if (Utilities|Operators|EqualEqual :A (Transformation|GetWorldRotation (Variables|/Game/Core/NPC/BP_Enemy.BP_Enemy_C|GetSplineMesh (Variables|Default|GetNPC))) :ErrorTolerance 1.0) :!label _label_2
                    (Sprite|SetFlipbook (Variables|/Game/Core/NPC/BP_Enemy.BP_Enemy_C|GetPaperFlipbook (Variables|Default|GetNPC)) "/Game/Core/Spirtes/Human/Melee/StabAttack.StabAttack")
                    (elif (Utilities|Operators|EqualEqual (Transformation|GetWorldRotation (Variables|/Game/Core/NPC/BP_Enemy.BP_Enemy_C|GetSplineMesh (Variables|Default|GetNPC))) "0.000000,180.000000,0.000000" 1.0)
                      (Sprite|SetFlipbook (Variables|/Game/Core/NPC/BP_Enemy.BP_Enemy_C|GetPaperFlipbook (Variables|Default|GetNPC)) "/Game/Core/Spirtes/Human/Melee/StabAttack.StabAttack")
                      (else
                        (Sprite|SetFlipbook (Variables|/Game/Core/NPC/BP_Enemy.BP_Enemy_C|GetPaperFlipbook (Variables|Default|GetNPC)) "/Game/Core/Spirtes/Human/Melee/StabAttack.StabAttack"))))
                  (CallFunction|PlayFlipbookRPC)
                  (Variables|Default|SetCondition false)
                  (Rendering|SetVisibility (Variables|/Game/Core/NPC/BP_Enemy.BP_Enemy_C|GetSplineMesh (Variables|Default|GetNPC)) false false)))
              (else
                (Variables|Default|SetPlayerHit? false)
                (goto _label_2))))
          (else
            (Variables|Default|SetCondition true)
            (Transformation|SetRelativeTransform (Variables|/Game/Core/NPC/BP_Enemy.BP_Enemy_C|GetSplineMesh (Variables|Default|GetNPC)) (Math|Transform|MakeTransform (.location (Transformation|GetRelativeTransform (Variables|/Game/Core/NPC/BP_Enemy.BP_Enemy_C|GetSplineMesh (Variables|Default|GetNPC)))) (.rotation (Transformation|GetRelativeTransform (Variables|/Game/Core/NPC/BP_Enemy.BP_Enemy_C|GetSplineMesh (Variables|Default|GetNPC)))) (Math|Vector|MakeVector (* (.range _weapondata_2) 0.32) (* (.width _weapondata_2) 0.32) 5.0)) false false)
            (Rendering|SetVisibility (Variables|/Game/Core/NPC/BP_Enemy.BP_Enemy_C|GetSplineMesh (Variables|Default|GetNPC)) true false)
            (Sprite|SetFlipbook (Variables|/Game/Core/NPC/BP_Enemy.BP_Enemy_C|GetPaperFlipbook (Variables|Default|GetNPC)) (Variables|/Game/Core/NPC/BP_Enemy.BP_Enemy_C|GetAttack%20Animation (Variables|Default|GetNPC)))
            (CallFunction|StopFlipbookRPC)))))))

(fn ConstructionScript)