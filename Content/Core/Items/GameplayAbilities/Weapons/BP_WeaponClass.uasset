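; Base weapon actor with a Paper2D sprite, leaving UseWeapon as an empty event, presumably for child weapons to override.
; On BeginPlay it loads its WeaponData from DB_Weapons by row name and adds to its Enchantments list.
; SetInUse toggles visibility, tick and actor collision, while always disabling the sprite's own collision.
; PassiveEffects runs each valid enchantment's PassiveEffect on the character.
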(event Custom|Passive%20Effects
  (for _array_element (Variables|Default|GetEnchantments)
    (Utilities|IsValid _array_element
      (:Is%20Valid
        (Default|PassiveEffect _array_element (Variables|Default|GetAs%20Bp%20Character))))))

(event Custom|SetInUse
  (params (InUse :type Boolean))
  ;[0.15 0.15 0.15 0.5] WeaponInUse?
  (Variables|Default|SetInUse InUse)
  (Collision|SetActorEnableCollision InUse)
  (Rendering|SetActorHiddenInGame (not InUse))
  (Actor|Tick|SetActorTickEnabled InUse)
  (Collision|SetCollisionEnabled (Variables|Default|GetPaperSprite) "NoCollision"))

(event Custom|UseWeapon
  (params (NPC%20Using? :type Boolean) (NPC :type BP%20Enemy%20Object%20Reference) (Player :type BP%20Character%20Object%20Reference)))

(event EventBeginPlay
  (bind _returnvalue (Utilities|GetDataTableRow "/Game/Core/Items/Weapons/DB_Weapons.DB_Weapons" (Variables|Default|GetItemDataRow))
    (:then
      (Variables|Default|SetWeaponData _returnvalue)
      (Utilities|Array|Add (Variables|Default|GetEnchantments) 0))
    (:RowNotFound
      (Development|PrintString "Hello"))))

(fn ConstructionScript)