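; BP_ThunderSpell is a weapon ability that calls down lightning on random tiles around the player.
; UseWeapon picks tiles within the weapon's width and range, keeps on-screen ones, and box-traces each for a target other than the player.
; Hits deal damage, play sound and character animation, and spawn a Skyfall_Spell bolt.
; A self-re-entering DoN caps attempts at SkyfallAmount, then resets if the aura exists; otherwise the lightning aura is applied.
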(event EventUseWeapon
  (params (NPC%20Using? :type Boolean) (NPC :type BP%20Enemy%20Object%20Reference))
  (bind _returnvalue (Viewport|GetViewportSize))
  (bind _weapondata (Variables|Default|GetWeaponData))
  (bind _weapondata_2 (Variables|Default|GetWeaponData))
  (Utilities|FlowControl|Sequence
    (:then_0
      (bind _asbp_character (Utilities|Casting|CastToBP_Character (Game|GetPlayerCharacter 0)))
      (Variables|Default|SetAs%20BP%20Character _asbp_character)
      (bind _asbp_controller (Utilities|Casting|CastToBP_Controller (Game|GetPlayerController 0)))
      (Utilities|FlowControl|DoN (Variables|Default|GetSkyfall%20Amount) :!label _label
        (:Exit
          (bind (_tilex _tiley) (Default|TiletoLocation (Variables|/Game/Core/BP_Controller.BP_Controller_C|GetTile%20Map _asbp_controller) (Math|Random|RandomIntegerinRange (- (Variables|/Game/Core/BP_Controller.BP_Controller_C|GetLeft/right _asbp_controller) (.width _weapondata_2)) (+ (Variables|/Game/Core/BP_Controller.BP_Controller_C|GetLeft/right _asbp_controller) (.width _weapondata_2))) (Math|Random|RandomIntegerinRange (- (Variables|/Game/Core/BP_Controller.BP_Controller_C|GetUp/Down _asbp_controller) (.range _weapondata_2)) (+ (Variables|/Game/Core/BP_Controller.BP_Controller_C|GetUp/Down _asbp_controller) (.range _weapondata_2)))))
          (if (Math|Boolean|ANDBoolean (> (.x (.ScreenLocation (Class|PlayerController|ProjectWorldLocationtoScreen (Game|GetPlayerController 0) (Math|Vector|MakeVector _tilex _tiley 5.0) false))) 0.0) (> (.y (.ScreenLocation (Class|PlayerController|ProjectWorldLocationtoScreen (Game|GetPlayerController 0) (Math|Vector|MakeVector _tilex _tiley 5.0) false))) 0.0) (< (.x (.ScreenLocation (Class|PlayerController|ProjectWorldLocationtoScreen (Game|GetPlayerController 0) (Math|Vector|MakeVector _tilex _tiley 5.0) false))) (.x _returnvalue)) (< (.y (.ScreenLocation (Class|PlayerController|ProjectWorldLocationtoScreen (Game|GetPlayerController 0) (Math|Vector|MakeVector _tilex _tiley 5.0) false))) (.y _returnvalue)))
            (bind _outactors (Actor|GetAllActorsOfClass "/Game/Core/Maps/TileMapGrid/BP_TilemapGen.BP_TilemapGen_C"))
            (bind _outhit (Collision|BoxTraceByChannel (Math|Vector|MakeVector _tilex _tiley 0.0) (Math|Vector|MakeVector _tilex _tiley 0.0) "24.000000,24.000000,0.000000" "0, 0, 0" "TraceTypeQuery1" false _outactors "None"))
            (if (!= (.hitactor _outhit) (Game|GetPlayerCharacter 0))
              (Utilities|IsValid (.hitactor _outhit)
                (:Is%20Valid
                  (Audio|PlaySound2D (.hitsound _weapondata) 1.0 1.0 0.0 0 0)
                  (bind _returnvalue_2 (Game|Damage|ApplyDamage (.hitactor _outhit) (.damage _weapondata) 0 0))
                  (CallFunction|DPS _returnvalue_2)
                  (Sprite|SetFlipbook (Variables|/Game/Core/BP_Character.BP_Character_C|GetPaperFlipbook (Variables|Default|GetAs%20BP%20Character)) "/Game/Core/Spirtes/Human/Melee/TrollDodge1.TrollDodge1")
                  (Components|Timeline|SetLooping (Variables|/Game/Core/BP_Character.BP_Character_C|GetPaperFlipbook (Variables|Default|GetAs%20BP%20Character)) false)
                  (Components|Timeline|PlayfromStart (Variables|/Game/Core/BP_Character.BP_Character_C|GetPaperFlipbook (Variables|Default|GetAs%20BP%20Character)))
                  (Game|SpawnActorfromClass "/Game/Core/Items/Projectiles/SpellEffects/Skyfall_Spell.Skyfall_Spell_C" (Math|Transform|MakeTransform (Math|Vector|MakeVector _tilex _tiley 5.0) "0, 0, 0" "1.000000,1.000000,1.000000") "Undefined" "MultiplyWithRoot" 0 "/Game/Core/Spirtes/Effects/Lightningboltwithcloud1.Lightningboltwithcloud1" 0)
                  (goto _label))
                (:Is%20Not%20Valid
                  (goto _label))))))))
    (:then_1
      (if (Utilities|IsValid (AssetData|GetAsset (Variables|/Game/Core/BP_Character.BP_Character_C|GetAura (Variables|Default|GetAs%20BP%20Character))))
        (goto _label Reset)
        (else
          (Class|NiagaraComponent|SetAsset (Variables|/Game/Core/BP_Character.BP_Character_C|GetAura (Variables|Default|GetAs%20BP%20Character)) "/Game/Core/assets/Effects/LightningAura.LightningAura" true))))))

(fn ConstructionScript
  (|CallParentFunction))