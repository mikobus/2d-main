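; BP_WeaponClass is a weapon actor that provides shared data, activation and damage-tracking logic, with an empty UseWeapon event.
; On BeginPlay it loads WeaponData from the DB_Weapons table using ItemDataRow.
; SetInUse toggles collision, visibility and tick together, so unused weapons stay hidden and inert.
; DPS plays the hit sound, adds damage to player 0's BP_Character total and sets InCombat through a DoOnce that is never reset here.
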(event Custom|UseWeapon
  (params (NPC%20Using? :type Boolean) (NPC :type BP%20Enemy%20Object%20Reference) (Player :type BP%20Character%20Object%20Reference)))

(event Custom|DPS
  (params (Damage%20Done :type Float%20%28double-precision%29))
  (bind _asbp_character (Utilities|Casting|CastToBP_Character (Game|GetPlayerCharacter 0)))
  (Audio|PlaySound2D (.HitSound (Utilities|Struct|BreakS_Weapon (Variables|Default|GetWeaponData))) 1.0 1.0 0.0 0 0)
  (Variables|/Game/Core/BP_Character.BP_Character_C|SetTotalDamageDone _asbp_character (+ (Variables|/Game/Core/BP_Character.BP_Character_C|GetTotalDamageDone _asbp_character) Damage%20Done))
  (Utilities|FlowControl|DoOnce false
    (:Completed
      (Variables|/Game/Core/BP_Character.BP_Character_C|SetInCombat? _asbp_character true))))

(event Custom|SetInUse
  (params (InUse :type Boolean))
  ;[0.15 0.15 0.15 0.5] WeaponInUse?
  (Variables|Default|SetInUse InUse)
  (Collision|SetActorEnableCollision InUse)
  (Rendering|SetActorHiddenInGame (not InUse))
  (Actor|Tick|SetActorTickEnabled InUse))

(event EventBeginPlay
  (bind _returnvalue (Utilities|GetDataTableRow "/Game/Core/Items/Weapons/DB_Weapons.DB_Weapons" (Variables|Default|GetItemDataRow))
    (:then
      (Variables|Default|SetWeaponData _returnvalue))
    (:RowNotFound
      (Development|PrintString "Hello"))))

(fn ConstructionScript)