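; BP_Upgrade is an upgrade chest pickup that offers its UpgradesInChest to the player character.
; On overlap with a BP_Character it closes any open pick UI, creates an Upgrade_PickUI with those upgrades, adds it to the viewport and destroys itself.
; Shortly after BeginPlay it caches the tilemap from BP_Gamemode, and the construction script stops its flipbook animation.
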(event EventBeginPlay
  (Utilities|FlowControl|Delay 0.2)
  (Utilities|FlowControl|Sequence
    (:then_0
      (bind _asbp_gamemode (Utilities|Casting|CastToBP_Gamemode (Game|GetGameMode)))
      (Variables|Default|SetTile%20Map (Default|GetTIlemap _asbp_gamemode)))))

(event Collision|EventActorBeginOverlap
  (params (OtherActor :type Actor%20Object%20Reference))
  (bind _asbp_character (Utilities|Casting|CastToBP_Character OtherActor))
  (Utilities|IsValid (Variables|/Game/Core/BP_Character.BP_Character_C|GetPickUIReference _asbp_character)
    (:Is%20Valid
      (Default|CloseUI _asbp_character))
    (:Is%20Not%20Valid
      _))
  (bind _returnvalue (Game|ConstructObjectfromClass _asbp_character "/Game/Core/Items/Upgrades/UpgradesUI/Upgrade_PickUI.Upgrade_PickUI_C" (Variables|Default|GetUpgradesInChest)))
  (UserInterface|Viewport|AddtoViewport _returnvalue 0)
  (Actor|DestroyActor))

(fn ConstructionScript
  (Audio|Components|Audio|Stop (Variables|Default|GetPaperFlipbook)))