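; Tilemap grid actor that loads the active tilemap as editable with rebuilt collision and tracks per-level enemy kill progress.
; NextLevel resets the count and totals EnemiesToSpawn across all EnemyTimeSpawner actors, while KillEvent updates the killed/total text display.
; LocationToTile and TileToLocation convert between world positions and tile indices relative to the actor's origin.
; Reaching the kill target triggers nothing; the House SleepBox collision logic is unconnected.
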(event Custom|KillEvent
  (bind _output_get (Variables|Default|SetEnemiesKilled (+ (Variables|Default|GetEnemiesKilled) 1)))
  (Rendering|Components|TextRender|SetText (Variables|Default|GetTextRender) (Utilities|Text|ToText(String) (Utilities|String|Append (Utilities|String|ToString(Integer) _output_get) "/" (Utilities|String|ToString(Integer) (Variables|Default|GetTotalEnemies)))))
  (if (>= (Variables|Default|GetEnemiesKilled) (Variables|Default|GetTotalEnemies))
    _))

(event Custom|NextLevel
  (Variables|Default|SetEnemiesKilled 0)
  (Variables|Default|SetTotalEnemies 0)
  (bind _outactors (Actor|GetAllActorsOfClass "/Game/Core/NPC/Spawners/EnemyTimeSpawner.EnemyTimeSpawner_C"))
  (for _array_element _outactors
    (bind _output_get (Variables|Default|SetTotalEnemies (+ (Variables|Default|GetTotalEnemies) (Variables|/Game/Core/NPC/Spawners/EnemyTimeSpawner.EnemyTimeSpawner_C|GetEnemiesToSpawn _array_element))))
    (Rendering|Components|TextRender|SetText (Variables|Default|GetTextRender) (Utilities|Text|ToText(String) (Utilities|String|Append "" "/" (Utilities|String|ToString(Integer) _output_get))))))

(event EventBeginPlay
  (bind _tilemap (Variables|Default|GetTileMap))
  (Utilities|FlowControl|Sequence
    (:then_0
      (Class|PaperTileMapComponent|SetTileMap (Variables|Default|GetTileMap) (Variables|Default|GetActiveTilemap))
      (Class|PaperTileMapComponent|MakeTileMapEditable _tilemap)
      (Class|PaperTileMapComponent|RebuildCollision _tilemap)
      (Variables|Default|SetBP%20TIlemapgrid self))))

(fn ConstructionScript)

(fn LocationtoTile
  (params (Location :type Vector))
  (bind (_x _y) (Math|Vector|BreakVector Location))
  (return (Math|Float|Truncate (/ (- _x (.x (Transformation|GetActorLocation))) 32.0)) (Math|Float|Truncate (/ (- _y (.y (Transformation|GetActorLocation))) 32.0))))

(fn TiletoLocation
  (params (LEFT/RIGHT :type Integer) (UP/DOWN :type Integer))
  (bind _returnvalue (Transformation|GetActorLocation))
  (bind _tilesize (Variables|Default|GetTileSize))
  (bind _returnvalue_2 (/ _tilesize 2.0))
  (bind _returnvalue_3 (select false _returnvalue_2 0.0))
  (Variables|Default|SetMapLeftRight UP/DOWN)
  (Variables|Default|SetMapUpDown LEFT/RIGHT)
  (return (+ (+ (* (Variables|Default|GetMapLeftRight) (Variables|Default|GetTileSize)) (.x _returnvalue)) _returnvalue_3) (+ _returnvalue_3 (+ (.y _returnvalue) (* (Variables|Default|GetMapUpDown) (Variables|Default|GetTileSize))))))