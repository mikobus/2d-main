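; BP_EventSelect is a Paper2D town trigger that opens the event UI when the player character touches it.
; After a short delay on BeginPlay, it gets the tile map from BP_Gamemode and moves itself to a hardcoded tile.
; Overlap with a BP_Character adds an EventUI widget to the viewport and destroys the actor, making it single-use.
; Its flipbook is stopped in the construction script.
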(event EventBeginPlay
  (Utilities|FlowControl|Delay 0.2)
  (Utilities|FlowControl|Sequence
    (:then_0
      (bind _asbp_gamemode (Utilities|Casting|CastToBP_Gamemode (Game|GetGameMode)))
      (bind _output_get (Variables|Default|SetTile%20Map (Default|GetTIlemap _asbp_gamemode)))
      (bind (_tilex _tiley) (Default|TiletoLocation _output_get 34 26))
      (Transformation|SetActorLocation (Math|Vector|MakeVector _tilex _tiley 5.0) false false))))

(event Collision|EventActorBeginOverlap
  (params (OtherActor :type Actor%20Object%20Reference))
  (bind _asbp_character (Utilities|Casting|CastToBP_Character OtherActor))
  (bind _returnvalue (Game|ConstructObjectfromClass _asbp_character "/Game/Core/LevelSwitches/TownItems/MapUI/EventUI.EventUI_C"))
  (UserInterface|Viewport|AddtoViewport _returnvalue 0)
  (Actor|DestroyActor))

(fn ConstructionScript
  (Audio|Components|Audio|Stop (Variables|Default|GetPaperFlipbook)))