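; BP_TrapSpawner is a trigger actor that scatters BP_Trap actors over random tiles when the player enters its Box.
; Shortly after BeginPlay it gets the TileMap from BP_Gamemode and moves to its configured tile.
; On overlap, it box-traces random tiles within its bounds, with persistent debug drawing, spawning only on unblocked ones.
; It retries without an attempt limit until ActorsToSpawn runs out, then destroys itself.
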(event OnComponentBeginOverlap(Box)
  (params (OverlappedComponent :type Primitive%20Component%20Object%20Reference) (OtherActor :type Actor%20Object%20Reference) (OtherComp :type Primitive%20Component%20Object%20Reference) (OtherBodyIndex :type Integer) (bFromSweep :type Boolean) (SweepResult :type Hit%20Result%20Structure%20%28by%20ref%29))
  ;[0.15 0.15 0.15 0.5] Trigger
  (if (== OtherActor (Game|GetPlayerCharacter 0))
    ;[0.15 0.15 0.15 0.5] check if spawned all
    (if (<= (Variables|Default|GetActorsToSpawn) 0) :!label _label
      (Actor|DestroyActor)
      (else
        ;[0.15 0.15 0.15 0.5] Random Tile
        (bind (_tilex _tiley) (Default|TiletoLocation (Variables|Default|GetTile%20Map) (Math|Random|RandomIntegerinRange (Variables|Default|GetMinSpawnLeftRight) (Variables|Default|GetMaxSpawnLeftRight)) (Math|Random|RandomIntegerinRange (Variables|Default|GetMinSpawnUpDown) (Variables|Default|GetMaxSpawnUpDown))))
        ;[0.15 0.15 0.15 0.5] Check if tile valid
        (bind _returnvalue (Collision|BoxTraceByChannel (Math|Vector|MakeVector _tilex _tiley 0.0) (Math|Vector|MakeVector _tilex _tiley 0.0) "8.000000,8.000000,0.000000" "0, 0, 0" "TraceTypeQuery1" false 0 "Persistent"))
        (if _returnvalue
          (goto _label)
          (else
            (Game|SpawnActorfromClass "/Game/Core/Enemies/Traps/BP_Trap.BP_Trap_C" (Math|Transform|MakeTransform (Math|Vector|MakeVector _tilex _tiley 0.0) "0, 0, 0" "1.000000,1.000000,1.000000") "Undefined" "MultiplyWithRoot" 0 0 0 0)
            ;[0.15 0.15 0.15 0.5] reduce actors
            (Variables|Default|SetActorsToSpawn (- (Variables|Default|GetActorsToSpawn) 1))
            (goto _label)))))))

(event EventBeginPlay
  (Utilities|FlowControl|Delay 0.2)
  (bind _asbp_gamemode (Utilities|Casting|CastToBP_Gamemode (Game|GetGameMode)))
  (bind _output_get (Variables|Default|SetTile%20Map (Variables|/Game/Core/BP_Gamemode.BP_Gamemode_C|GetTileMap _asbp_gamemode)))
  (bind (_tilex _tiley) (Default|TiletoLocation _output_get (Variables|Default|GetTrapSpawnerLeftRight) (Variables|Default|GetTrapSpawnerUpDown)))
  (Transformation|SetActorLocation (Math|Vector|MakeVector _tilex _tiley 0.0) false false))

(fn ConstructionScript)