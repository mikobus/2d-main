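; BP_MapExit is a map exit trigger that ends play on the map when the player reaches it.
; Its Box overlap responds only to the player character's capsule.
; It then disables input on BP_Controller, adds a new WB_MapExit widget to the viewport and destroys every BP_Enemy actor in the world.
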(event OnComponentBeginOverlap(Box)
  (params (OverlappedComponent :type Primitive%20Component%20Object%20Reference) (OtherActor :type Actor%20Object%20Reference) (OtherComp :type Primitive%20Component%20Object%20Reference) (OtherBodyIndex :type Integer) (bFromSweep :type Boolean) (SweepResult :type Hit%20Result%20Structure%20%28by%20ref%29))
  (if (== OtherComp (Variables|/Script/Engine.Character|GetCapsuleComponent (Game|GetPlayerCharacter 0)))
    (bind _asbp_controller (Utilities|Casting|CastToBP_Controller (Game|GetPlayerController 0)))
    (Input|DisableInput _asbp_controller 0)
    (bind _returnvalue (Game|ConstructObjectfromClass "/Game/Core/Tilemaps/MapObjects/Exit/WB_MapExit.WB_MapExit_C"))
    (UserInterface|Viewport|AddtoViewport _returnvalue 0)
    (bind _outactors (Actor|GetAllActorsOfClass "/Game/Core/NPC/BP_Enemy.BP_Enemy_C"))
    (for _array_element _outactors
      (Actor|DestroyActor _array_element))))

(fn ConstructionScript)