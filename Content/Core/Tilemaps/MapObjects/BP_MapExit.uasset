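; BP_MapExit is a map exit trigger that sends the player back to the Lobby level.
; When the player's capsule overlaps its box, SetStats runs, then the Lobby level opens.
; SetStats copies the BP_Character's abilities, gold, health, attack stats, flipbook and weapon sprite, plus its controller's attack movement, into CurrentGameInstance so they persist across the level change.
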(event OnComponentBeginOverlap(Box)
  (params (OverlappedComponent :type Primitive%20Component%20Object%20Reference) (OtherActor :type Actor%20Object%20Reference) (OtherComp :type Primitive%20Component%20Object%20Reference) (OtherBodyIndex :type Integer) (bFromSweep :type Boolean) (SweepResult :type Hit%20Result%20Structure%20%28by%20ref%29))
  (if (== OtherComp (Variables|/Script/Engine.Character|GetCapsuleComponent (Game|GetPlayerCharacter 0)))
    (Utilities|FlowControl|Sequence
      (:then_0
        (CallFunction|SetStats))
      (:then_1
        (Game|OpenLevel(byName) "Lobby")))))

(fn ConstructionScript)

(fn SetStats
  (bind _returnvalue (Actor|GetActorOfClass "/Game/Core/BP_Character.BP_Character_C"))
  (bind _ascurrent_game_instance (Utilities|Casting|CastToCurrentGameInstance (Game|GetGameInstance)))
  (Variables|/Game/Core/Events/CurrentGameInstance.CurrentGameInstance_C|SetAbilities _ascurrent_game_instance (Variables|/Game/Core/BP_Character.BP_Character_C|GetAbilities _returnvalue))
  (Variables|/Game/Core/Events/CurrentGameInstance.CurrentGameInstance_C|SetFlipbook _ascurrent_game_instance (Class|PaperFlipbookComponent|GetFlipbook (Variables|/Game/Core/BP_Character.BP_Character_C|GetPaperFlipbook _returnvalue)))
  (Variables|/Game/Core/Events/CurrentGameInstance.CurrentGameInstance_C|SetGold _ascurrent_game_instance (Variables|/Game/Core/BP_Character.BP_Character_C|GettotalGold _returnvalue))
  (Variables|/Game/Core/Events/CurrentGameInstance.CurrentGameInstance_C|SetPlayerHealth _ascurrent_game_instance (Variables|/Game/Core/BP_Character.BP_Character_C|GetHealth _returnvalue))
  (Variables|/Game/Core/Events/CurrentGameInstance.CurrentGameInstance_C|SetAttackDamage _ascurrent_game_instance (Variables|/Game/Core/BP_Character.BP_Character_C|GetAttackDamage _returnvalue))
  (Variables|/Game/Core/Events/CurrentGameInstance.CurrentGameInstance_C|SetAttackRange _ascurrent_game_instance (Variables|/Game/Core/BP_Character.BP_Character_C|GetAttackRange _returnvalue))
  (Variables|/Game/Core/Events/CurrentGameInstance.CurrentGameInstance_C|SetAttackWidth _ascurrent_game_instance (Variables|/Game/Core/BP_Character.BP_Character_C|GetAttackWidth _returnvalue))
  (Variables|/Game/Core/Events/CurrentGameInstance.CurrentGameInstance_C|SetWeaponMesh _ascurrent_game_instance (Sprite|GetSprite (Variables|/Game/Core/BP_Character.BP_Character_C|GetWeapon _returnvalue)))
  (Variables|/Game/Core/Events/CurrentGameInstance.CurrentGameInstance_C|SetAttackMovement _ascurrent_game_instance (Variables|/Game/Core/BP_Controller.BP_Controller_C|GetAttackMovementWeapon (Variables|/Game/Core/BP_Character.BP_Character_C|GetControllerRef _returnvalue))))