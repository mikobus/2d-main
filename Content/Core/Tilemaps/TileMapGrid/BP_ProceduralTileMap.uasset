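; Procedural tilemap level actor that paints a Plains or Bridge layout on BeginPlay according to MapType.
; GenerateMap lays border walls, adds Bridge's dividing walls and layer-2 side fills, cuts fixed corridors, then rebuilds collision.
; OpenGate retries random tiles with a box trace until one is clear, then spawns BP_MapExit there.
; A randomly seeded Perlin FastNoise is created, but the cave-noise pass using it is disconnected, so layouts are fixed.
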(event Custom|GenerateMap
  (bind _tiles (Variables|Default|GetTiles))
  (bind _tiles_2 (Variables|Default|GetTiles))
  (bind _output (Utilities|Array|Get(acopy) _tiles_2 2))
  (bind _output_2 (Utilities|Array|Get(acopy) _tiles 2))
  (switch Utilities|FlowControl|Switch|SwitchonE_MapTypes (Variables|Default|GetMapType)
    (:NewEnumerator0
      ;[0.15 0.15 0.15 0.5] Make Walls
      (for _index (range 0 (- (Variables|Default|GetMapSizeHeight) 1))
        (for _index_2 (range 0 (- (Variables|Default|GetMapSizeWidth) 1))
          (if (Math|Boolean|ORBoolean (== _index 0) (== _index (- (Variables|Default|GetMapSizeHeight) 1)) (== _index_2 0) (== _index_2 (- (Variables|Default|GetMapSizeWidth) 1)))
            (Variables|Default|SetTileChosen 1)
            (Utilities|Array|AddUnique (Variables|Default|GetMapWalls) (Math|Vector2D|MakeVector2D (Math|Conversions|ToFloat(Integer) _index_2) (Math|Conversions|ToFloat(Integer) _index)))
            (else
              (Variables|Default|SetTileChosen 0)))
          (Class|PaperTileMapComponent|SetTile (Variables|Default|GetTileMap) _index_2 _index 0 (Utilities|Array|Get(acopy) (Variables|Default|GetTiles) (Variables|Default|GetTileChosen)))))
      ;[0.15 0.15 0.15 0.5] Noise
      (for _index_3 (range 0 15)
        (for _index_4 (range 9 11)
          (Class|PaperTileMapComponent|SetTile (Variables|Default|GetTileMap) _index_4 _index_3 0 (Utilities|Array|Get(acopy) (Variables|Default|GetTiles)))))
      (for _index_5 (range 15 21)
        (for _index_6 (range 9 11)
          (Class|PaperTileMapComponent|SetTile (Variables|Default|GetTileMap) _index_6 _index_5 0 (Utilities|Array|Get(acopy) (Variables|Default|GetTiles)))))
      (Class|PaperTileMapComponent|RebuildCollision (Variables|Default|GetTileMap)))
    (:NewEnumerator3
      ;[0.15 0.15 0.15 0.5] GenBridge
      ;;[0.15 0.15 0.15 0.5] Make Walls
      (for _index_7 (range 0 (- (Variables|Default|GetMapSizeHeight) 1))
        (for _index_8 (range 0 (- (Variables|Default|GetMapSizeWidth) 1))
          (if (Math|Boolean|ORBoolean (== _index_7 0) (== _index_7 (- (Variables|Default|GetMapSizeHeight) 1)) (== _index_8 0) (== _index_8 (- (Variables|Default|GetMapSizeWidth) 1)) (== _index_8 11) (== _index_8 29))
            (Variables|Default|SetTileChosen 1)
            (else
              (Variables|Default|SetTileChosen 0)))
          (Class|PaperTileMapComponent|SetTile (Variables|Default|GetTileMap) _index_8 _index_7 0 (Utilities|Array|Get(acopy) (Variables|Default|GetTiles) (Variables|Default|GetTileChosen)))))
      (for _index_9 (range 1 (- (Variables|Default|GetMapSizeHeight) 2))
        (if (Utilities|Array|IsValidIndex (Variables|Default|GetTiles) 2)
          (for _index_10 (range 1 10)
            (Class|PaperTileMapComponent|SetTile (Variables|Default|GetTileMap) _index_10 _index_9 2 (Utilities|Struct|MakePaperTileInfo (.tileindex _output_2) (.tileset _output_2) false true false)))
          (for _index_11 (range 30 (- (Variables|Default|GetMapSizeWidth) 2))
            (Class|PaperTileMapComponent|SetTile (Variables|Default|GetTileMap) _index_11 _index_9 2 (Utilities|Struct|MakePaperTileInfo (.tileindex _output) (.tileset _output) false true false)))))
      (for _index_12 (range 0 15)
        (for _index_13 (range 19 21)
          (Class|PaperTileMapComponent|SetTile (Variables|Default|GetTileMap) _index_13 _index_12 0 (Utilities|Array|Get(acopy) (Variables|Default|GetTiles)))))
      (for _index_14 (range 25 40)
        (for _index_15 (range 19 21)
          (Class|PaperTileMapComponent|SetTile (Variables|Default|GetTileMap) _index_15 _index_14 0 (Utilities|Array|Get(acopy) (Variables|Default|GetTiles)))))
      (Class|PaperTileMapComponent|RebuildCollision (Variables|Default|GetTileMap)))))

(event EventBeginPlay
  (Variables|Default|SetMapChosen? true)
  (|CallParentFunction)
  (bind _returnvalue (Game|ConstructObjectfromClass "/Script/FastNoiseGenerator.FastNoiseWrapper"))
  (bind _output_get (Variables|Default|SetNoiseGen _returnvalue))
  (Class|FastNoiseWrapper|SetupFastNoise _output_get "Perlin" (Math|Random|RandomIntegerinRange 1111 1023109) 0.1 "Quintic" "FBM" 3 2.0 1.0 0.5 "Euclidean" "CellValue")
  (CallFunction|GenerateMap))

(event EventOpenGate
  (|CallParentFunction)
  (bind (_tilex _tiley) (CallFunction|TiletoLocation (Math|Random|RandomIntegerinRange 12 28) (Math|Random|RandomIntegerinRange 1 39) :!label _label))
  (bind _returnvalue (Collision|BoxTraceByChannel (Math|Vector|MakeVector _tilex _tiley 0.0) (Math|Vector|MakeVector _tilex _tiley 0.0) "8.000000,8.000000,0.000000" "0, 0, 0" "TraceTypeQuery1" false 0 "None" false))
  (if _returnvalue
    (goto _label)
    (else
      (Game|SpawnActorfromClass "/Game/Core/Tilemaps/MapObjects/BP_MapExit.BP_MapExit_C" (Math|Transform|MakeTransform (Math|Vector|MakeVector _tilex _tiley -14.0) "0, 0, 0" "1.000000,1.000000,1.000000") "Undefined" "MultiplyWithRoot" 0 0))))

(fn ConstructionScript
  (|CallParentFunction))

(fn CountNeighbors
  (params (X :type Integer) (Y :type Integer))
  (bind _tiles (Variables|Default|GetTiles))
  (bind _output (Utilities|Array|Get(acopy) _tiles 4))
  (bind _output_2 (Utilities|Array|Get(acopy) _tiles 1))
  (for _array_element (Variables|Default|GetSurroundingTiles)
    (if (or (and (== (.tileindex (Class|PaperTileMapComponent|GetTile (Variables|Default|GetTileMap) (Math|Float|Truncate (+ (.x _array_element) X)) (Math|Float|Truncate (+ (.y _array_element) Y)))) (.tileindex _output_2)) (== (.tileset _output_2) (.tileset (Class|PaperTileMapComponent|GetTile (Variables|Default|GetTileMap) (Math|Float|Truncate (+ (.x _array_element) X)) (Math|Float|Truncate (+ (.y _array_element) Y)))))) (and (== (.tileindex _output) (.tileindex (Class|PaperTileMapComponent|GetTile (Variables|Default|GetTileMap) (Math|Float|Truncate (+ (.x _array_element) X)) (Math|Float|Truncate (+ (.y _array_element) Y))))) (== (.tileset _output) (.tileset (Class|PaperTileMapComponent|GetTile (Variables|Default|GetTileMap) (Math|Float|Truncate (+ (.x _array_element) X)) (Math|Float|Truncate (+ (.y _array_element) Y)))))))
      (Variables|Default|SetWallCount (+ (Variables|Default|GetWallCount) 1))))
  (return (Variables|Default|GetWallCount)))

(fn PerlinNoise2D
  (params (X :type Float%20%28double-precision%29) (Y :type Float%20%28double-precision%29) (Scale :type Float%20%28double-precision%29))
  (return (/ (+ (Class|KismetMathLibrary|PerlinNoise1D (* X Scale)) (Class|KismetMathLibrary|PerlinNoise1D (* Y Scale))) 2.0)))