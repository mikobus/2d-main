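; Tilemap actor with an event trigger and gate that leads the player into procedurally generated levels.
; Unless day 3 debt is unpaid, the event box shows EventUI, and MapChosen removes it and opens the gate.
; Crossing the gate box closes it by tile editing, clears enemies, increments the level, then spawns BP_ProceduralTileMap and a level-scaled enemy spawner.
; Helper functions convert between world locations and tile coordinates.
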(event OnComponentBeginOverlap(GateBox)
  (params (OverlappedComponent :type Primitive%20Component%20Object%20Reference) (OtherActor :type Actor%20Object%20Reference) (OtherComp :type Primitive%20Component%20Object%20Reference) (OtherBodyIndex :type Integer) (bFromSweep :type Boolean) (SweepResult :type Hit%20Result%20Structure%20%28by%20ref%29))
  (bind _gatetiles (Variables|Default|GetGateTiles))
  (if (== OtherComp (Variables|/Script/Engine.Character|GetCapsuleComponent (Game|GetPlayerCharacter 0)))
    (CallFunction|MapComplete true)
    (Rendering|SetVisibility (Variables|Default|GetGateTiles) true false)
    (Collision|SetCollisionEnabled (Variables|Default|GetGateBox) "NoCollision")
    (Collision|SetCollisionEnabled (Variables|Default|GetGateTiles) "QueryAndPhysics")
    (Class|PaperTileMapComponent|SetTile _gatetiles 1 0 0 (Utilities|Struct|MakePaperTileInfo 2 "/Game/Core/Spirtes/Tilesets/Grasslands_TileSet.Grasslands_TileSet" false false false))
    (Class|PaperTileMapComponent|RebuildCollision _gatetiles)))

(event OnComponentBeginOverlap(EventBox)
  (params (OverlappedComponent :type Primitive%20Component%20Object%20Reference) (OtherActor :type Actor%20Object%20Reference) (OtherComp :type Primitive%20Component%20Object%20Reference) (OtherBodyIndex :type Integer) (bFromSweep :type Boolean) (SweepResult :type Hit%20Result%20Structure%20%28by%20ref%29))
  (bind _asbp_gamemode (Utilities|Casting|CastToBP_Gamemode (Game|GetGameMode)))
  (if (not (and (== (Variables|/Game/Core/BP_Gamemode.BP_Gamemode_C|GetCurrentDay _asbp_gamemode) 3) (not (Variables|Default|GetDebtPaid?))))
    (if (Utilities|Operators|EqualEqual (Transformation|GetActorLocation OtherActor) (Transformation|GetActorLocation (Game|GetPlayerCharacter 0)) 5.0)
      (Collision|SetCollisionEnabled (Variables|Default|GetEventBox) "NoCollision")
      (bind _asbp_character (Utilities|Casting|CastToBP_Character OtherActor))
      (bind _returnvalue (Game|ConstructObjectfromClass _asbp_character "/Game/Core/Events/MapUI/EventUI.EventUI_C"))
      (UserInterface|Viewport|AddtoViewport _returnvalue 0)
      (Widget|SetVisibility (Variables|/Game/Core/Interface/GoldAndUI/I_Interface.I_Interface_C|GetDay (Variables|/Game/Core/BP_Character.BP_Character_C|GetInterfaceReference _asbp_character)) "Hidden")
      (Widget|SetVisibility (Variables|/Game/Core/Interface/GoldAndUI/I_Interface.I_Interface_C|GetDebt (Variables|/Game/Core/BP_Character.BP_Character_C|GetInterfaceReference _asbp_character)) "Hidden"))))

(event Custom|MapChosen
  (Input|EnableInput (Game|GetPlayerController 0) 0)
  (Widget|RemovefromParent (stale OnComponentBeginOverlap(EventBox) _returnvalue))
  (CallFunction|OpenGate)
  (Variables|Default|SetDebtPaid? false))

(event Custom|OpenGate
  (bind _gatetiles (Variables|Default|GetGateTiles))
  (Class|PaperTileMapComponent|MakeTileMapEditable _gatetiles)
  (Class|PaperTileMapComponent|SetTile _gatetiles 1 0 0 (Utilities|Struct|MakePaperTileInfo -1 "/Game/Core/Spirtes/Tilesets/BrickTiles_TileSet1.BrickTiles_TileSet1" false false false))
  (Class|PaperTileMapComponent|RebuildCollision _gatetiles))

(event Custom|MapComplete
  (params (IncreaseLevel? :type Boolean))
  (Utilities|IsValid (Variables|Default|GetEventBox)
    (:Is%20Valid
      (bind _outactors (Actor|GetAllActorsOfClass "/Game/Core/NPC/BP_Enemy.BP_Enemy_C"))
      (for _array_element _outactors
        (Utilities|IsValid _array_element
          (:Is%20Valid
            (Actor|DestroyActor _array_element))))
      (if IncreaseLevel?
        (bind _asbp_gamemode (Utilities|Casting|CastToBP_Gamemode (Game|GetGameMode)))
        (bind _output_get (Variables|/Game/Core/BP_Gamemode.BP_Gamemode_C|SetCurrent%20Level _asbp_gamemode (+ (Variables|/Game/Core/BP_Gamemode.BP_Gamemode_C|GetCurrent%20Level _asbp_gamemode) 1)))
        (bind _output_get_2 (Variables|Default|SetCurrentLevel _output_get)))
      (Development|PrintString (Utilities|String|Append "Current Level: " (Utilities|String|ToString(Integer) _output_get_2)))
      (Game|SpawnActorfromClass "/Game/Core/Tilemaps/TileMapGrid/BP_ProceduralTileMap.BP_ProceduralTileMap_C" (Math|Transform|MakeTransform (Math|Vector|MakeVector (+ (.x (Transformation|GetWorldLocation (Variables|Default|GetEventBox))) 64.0) 3.2e+02 0.0) "0, 0, 0" "1.000000,1.000000,1.000000") "Undefined" "MultiplyWithRoot" 0 "/Game/Core/Tilemaps/Levels/GENmap.GENmap" (Variables|Default|GetMapType) (Variables|Default|GetTiles) (Variables|Default|GetCurrentLevel) 0)
      (Game|SpawnActorfromClass "/Game/Core/NPC/Spawners/EnemyTimeSpawner.EnemyTimeSpawner_C" (Math|Transform|MakeTransform "0, 0, 0" "0, 0, 0" "1.000000,1.000000,1.000000") "Undefined" "MultiplyWithRoot" 0 (* (Variables|Default|GetCurrentLevel) 10) (Variables|Default|GetCurrentLevel) (Variables|Default|GetBP%20TIlemapgrid) 5.0 "Friendly" 0))))

(event EventBeginPlay
  (bind _tilemap (Variables|Default|GetTileMap))
  (Class|PaperTileMapComponent|SetTileMap (Variables|Default|GetTileMap) (Variables|Default|GetActiveTilemap))
  (Class|PaperTileMapComponent|MakeTileMapEditable _tilemap)
  (Class|PaperTileMapComponent|RebuildCollision _tilemap)
  (Variables|Default|SetBP%20TIlemapgrid self)
  (Class|PaperTileMapComponent|SetTileMap (Variables|Default|GetGateTiles) "/Game/Core/Tilemaps/MapObjects/LevelGates.LevelGates"))

(fn ConstructionScript)

(fn LocationtoTile
  (params (Location :type Vector))
  (bind _mapwidth (Variables|Default|GetMapWidth))
  (bind _mapheight (Variables|Default|GetMapHeight))
  (bind _output_get (Variables|Default|SetLocation Location))
  (return (/ (Math|Float|Floor (* _mapwidth (/ (- (.x _output_get) (.x (Transformation|GetActorLocation))) _mapwidth))) 32) (/ (Math|Float|Floor (* _mapheight (/ (- (.y _output_get) (.y (Transformation|GetActorLocation))) _mapheight))) 32)))

(fn TiletoLocation
  (params (LEFT/RIGHT :type Integer) (UP/DOWN :type Integer))
  (bind _returnvalue (Transformation|GetActorLocation))
  (bind _tilesize (Variables|Default|GetTileSize))
  (bind _returnvalue_2 (/ _tilesize 2.0))
  (bind _returnvalue_3 (select false _returnvalue_2 0.0))
  (Variables|Default|SetMapWidth UP/DOWN)
  (Variables|Default|SetMapHeight LEFT/RIGHT)
  (return (+ (+ (* (Variables|Default|GetMapWidth) (Variables|Default|GetTileSize)) (.x _returnvalue)) _returnvalue_3) (+ _returnvalue_3 (+ (.y _returnvalue) (* (Variables|Default|GetMapHeight) (Variables|Default|GetTileSize))))))