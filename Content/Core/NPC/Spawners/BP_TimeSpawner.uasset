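; Enemy spawner that pre-creates a pool of BP_MeleeNPC actors at BeginPlay and places them around the player during play.
; Each MovementTick, while spawning is enabled, it rerolls random tiles in a band offset from the player's UpDown coordinate until one is off-screen.
; If a box trace there finds no blocker, it activates a free pooled enemy and adds the player's CurrentLevel to its Health.
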(event Custom|Spawn%20Pool
  (if (> (Variables|Default|GetEnemiesToSpawn) 0)
    (for _index (range 0 (Variables|Default|GetEnemiesToSpawn))
      (bind _returnvalue (Game|SpawnActorfromClass "/Game/Core/NPC/BP_MeleeNPC.BP_MeleeNPC_C" (Math|Transform|MakeTransform (Math|Vector|MakeVector 0.0 0.0 5.0) "0, 0, 0" "1.000000,1.000000,1.000000") "Undefined" "MultiplyWithRoot" 0 8 1 2 0))
      (Utilities|Array|AddUnique (Variables|Default|GetEnemyPool) _returnvalue))
    (for _array_element (Variables|Default|GetEnemyPool)
      (Default|SetinUse _array_element false))))

(event EventBeginPlay
  (Utilities|FlowControl|Delay 0.2)
  (|CallParentFunction)
  (CallFunction|SpawnPool))

(event EventMovementTick
  (bind _returnvalue (Viewport|GetViewportSize))
  ;[0.15 0.15 0.15 0.5] Every movement spawns
  (if (Variables|Default|GetSpawningEnabled?)
    (if (not (<= (Variables|Default|GetEnemiesToSpawn) 0))
      (bind (_updown _leftright) (Default|LocationtoTile (Variables|Default|GetTile%20Map) (Transformation|GetActorLocation (Game|GetPlayerCharacter 0))))
      (Variables|Default|SetPlayer%20Up%20Down _updown)
      (Variables|Default|SetPlayer%20LeftRight _leftright)
      ;[0.15 0.15 0.15 0.5] Get Random Tile
      (bind (_tilex _tiley) (Default|TiletoLocation (Variables|Default|GetTile%20Map) (Math|Random|RandomIntegerinRange 8 30) (Math|Random|RandomIntegerinRange (+ (Variables|Default|GetPlayer%20Up%20Down) 15) (+ (Variables|Default|GetPlayer%20Up%20Down) 40)) :!label _label))
      (if (Math|Boolean|ANDBoolean (> (.x (.ScreenLocation (Class|PlayerController|ProjectWorldLocationtoScreen (Game|GetPlayerController 0) (Math|Vector|MakeVector _tilex _tiley 5.0) false))) 0.0) (> (.y (.ScreenLocation (Class|PlayerController|ProjectWorldLocationtoScreen (Game|GetPlayerController 0) (Math|Vector|MakeVector _tilex _tiley 5.0) false))) 0.0) (< (.x (.ScreenLocation (Class|PlayerController|ProjectWorldLocationtoScreen (Game|GetPlayerController 0) (Math|Vector|MakeVector _tilex _tiley 5.0) false))) (.x _returnvalue)) (< (.y (.ScreenLocation (Class|PlayerController|ProjectWorldLocationtoScreen (Game|GetPlayerController 0) (Math|Vector|MakeVector _tilex _tiley 5.0) false))) (.y _returnvalue)))
        (goto _label)
        (else
          ;[0.15 0.15 0.15 0.5] Check if Collides and if not spawn actor
          (bind _returnvalue_2 (Collision|BoxTraceByChannel (Math|Vector|MakeVector _tilex _tiley 5.0) (Math|Vector|MakeVector _tilex _tiley 5.0) (Math|Vector|MakeVector 8.0 8.0 5.0) "0, 0, 0" "TraceTypeQuery1" false 0 "None"))
          (if (not _returnvalue_2)
            (bind _array_element (CallFunction|SpawnfromPool (Math|Vector|MakeVector _tilex _tiley 5.0)))
            (bind _asbp_character (Utilities|Casting|CastToBP_Character (Game|GetPlayerCharacter 0)))
            (Variables|/Game/Core/NPC/BP_Enemy.BP_Enemy_C|SetHealth _array_element (+ (Variables|/Game/Core/NPC/BP_Enemy.BP_Enemy_C|GetHealth _array_element) (Variables|/Game/Core/BP_Character.BP_Character_C|GetCurrentLevel _asbp_character)))))))))

(fn ConstructionScript)

(fn FindFirstAvailableActor
  (for _array_element (Variables|Default|GetEnemyPool)
    (if (not (Variables|/Game/Core/NPC/BP_Enemy.BP_Enemy_C|GetInUse _array_element))
      (return _array_element))))

(fn SpawnfromPool
  (params (Spawn%20Location :type Vector))
  (bind _array_element (CallFunction|FindFirstAvailableActor))
  (Utilities|IsValid _array_element
    (:Is%20Valid
      (Transformation|SetActorLocation _array_element Spawn%20Location false false)
      (Default|SetinUse _array_element true)
      (return _array_element))))

(fn AddActorstoPool
  (bind _outactors (Actor|GetAllActorsOfClass "/Game/Core/NPC/BP_Enemy.BP_Enemy_C"))
  (for _array_element _outactors
    (Utilities|Array|AddUnique (Variables|Default|GetEnemyPool) _array_element))
  (return))