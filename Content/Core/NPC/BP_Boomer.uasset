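; Boomer enemy NPC that chases the player and readies an explosion once in range.
; MoveToPlayer hides the zone marker, follows and locates the player, then either marks the attack zone or resets the weapon sprite's tint and scale.
; MarkAttackZone stops movement, snaps the marker mesh to the Boomer's own tile via TileMap, and sets ExplosionReady.
; The event graph is empty, and the detonation is not handled here.
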(event EventBeginPlay)

(event Collision|EventActorBeginOverlap
  (params (OtherActor :type Actor%20Object%20Reference)))

(event EventTick
  (params (DeltaSeconds :type Float%20%28single-precision%29)))

(fn ConstructionScript)

(fn MarkAttackZone
  (bind _tile_map (Variables|Default|GetTile%20Map))
  (bind _staticmesh (Variables|Default|GetStaticMesh))
  (Variables|Default|SetCanMove false)
  (bind (_updown _leftright) (Default|LocationtoTile _tile_map (Transformation|GetActorLocation)))
  (bind (_tilex _tiley) (Default|TiletoLocation _tile_map _leftright _updown))
  (Rendering|SetVisibility _staticmesh true false)
  (Transformation|SetWorldLocation _staticmesh (Math|Vector|MakeVector _tilex _tiley 0.0) false false)
  (Variables|Default|SetExplosionReady true))

(fn MovetoPlayer
  ;[0.15 0.15 0.15 0.5] Enemy is NOT in range -> Move To Player
  (Rendering|SetVisibility (Variables|Default|GetStaticMesh) false false)
  (CallFunction|FollowPlayer)
  (CallFunction|FindPlayer)
  ;;[0.15 0.15 0.15 0.5] if player is in range enemy moves mark the zone
  (bind _newparam (CallFunction|IsPlayerinRange))
  (if _newparam
    (CallFunction|MarkAttackZone)
    (else
      (Sprite|SetSpriteColor (Variables|Default|GetWeapon) "(R=1.000000,G=1.000000,B=1.000000,A=1.000000)")
      (Transformation|SetRelativeScale3D (Variables|Default|GetWeapon) "0.500000,0.500000,0.500000"))))