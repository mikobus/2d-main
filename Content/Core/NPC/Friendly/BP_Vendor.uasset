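; Friendly vendor NPC that offers randomly picked weapons through a store UI.
; After a short delay on begin play, it snaps to a fixed tile on the player's tile map and fills its item slots with random DB_Weapons rows.
; Player overlap sets a flag on the controller, and VendorScreen opens a single I_Vendor widget.
; Leaving overlap clears the flag and closes the store, hiding the cursor unless the inventory is visible.
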(event Custom|VendorScreen
  (if (not (Variables|Default|GetStoreVisible))
    (bind _asbp_character (Utilities|Casting|CastToBP_Character (Game|GetPlayerCharacter 0)))
    (bind _returnvalue (Game|ConstructObjectfromClass _asbp_character "/Game/Core/NPC/Friendly/VendorInterface/I_Vendor.I_Vendor_C"))
    (bind _output_get (Variables|Default|SetStoreUi _returnvalue))
    (UserInterface|Viewport|AddtoViewport _output_get 0)
    (Variables|Default|SetStoreVisible true)))

(event EventBeginPlay
  (Utilities|FlowControl|Delay 0.2)
  (Utilities|FlowControl|Sequence
    (:then_0
      (bind _asbp_character (Utilities|Casting|CastToBP_Character (Game|GetPlayerCharacter 0)))
      (Variables|Default|SetTile%20Map (Variables|/Game/Core/BP_Character.BP_Character_C|GetTile%20Map _asbp_character)))
    (:then_1
      (bind (_tilex _tiley) (Default|TiletoLocation (Variables|Default|GetTile%20Map) 15 7))
      (Transformation|SetActorLocation (Math|Vector|MakeVector _tilex _tiley 5.0) false false))
    (:then_2
      (for (_ _array_index) (Variables|Default|GetVendorItems)
        (Utilities|Array|SetArrayElem (Variables|Default|GetVendorItems) _array_index (Utilities|Struct|MakeS_Slots (Utilities|Struct|MakeDataTableRowHandle "/Game/Core/Weapons/DB_Weapons.DB_Weapons" (Utilities|String|StringToName (Utilities|String|ToString(Integer) (Math|Random|RandomIntegerinRange 1 6))))))))))

(event Collision|EventActorBeginOverlap
  (params (OtherActor :type Actor%20Object%20Reference))
  (if (== OtherActor (Game|GetPlayerCharacter 0))
    (bind _asbp_controller (Utilities|Casting|CastToBP_Controller (Game|GetPlayerController 0)))
    (Variables|/Game/Core/BP_Controller.BP_Controller_C|SetOverlappingVendor? _asbp_controller true)
    (Development|PrintString "overlapping")))

(event Collision|EventActorEndOverlap
  (params (OtherActor :type Actor%20Object%20Reference))
  (if (== OtherActor (Game|GetPlayerCharacter 0))
    (bind _asbp_controller (Utilities|Casting|CastToBP_Controller (Game|GetPlayerController 0)))
    (Variables|/Game/Core/BP_Controller.BP_Controller_C|SetOverlappingVendor? _asbp_controller false)
    (bind _asbp_character (Utilities|Casting|CastToBP_Character (Game|GetPlayerCharacter 0)))
    (Utilities|IsValid (stale Custom|VendorScreen _returnvalue)
      (:Is%20Valid
        (Widget|RemovefromParent (stale Custom|VendorScreen _returnvalue))
        (Variables|Default|SetStoreVisible false)
        (if (not (Widget|IsVisible (Variables|/Game/Core/Inventory/BPC_Inventory.BPC_Inventory_C|GetInventoryReference (Variables|/Game/Core/BP_Character.BP_Character_C|GetBPC_Inventory _asbp_character))))
          (Variables|/Script/Engine.PlayerController|SetbShowMouseCursor (stale Collision|EventActorBeginOverlap _asbp_controller) false))))))

(fn ConstructionScript)