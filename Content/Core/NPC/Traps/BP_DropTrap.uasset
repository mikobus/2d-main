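; BP_DropTrap is a 2D trap that damages the player on contact with its Box trigger.
; When the player character's capsule begins overlapping the box, it replays the PaperFlipbook animation once from the first frame and applies fixed damage immediately.
; The construction script stops the flipbook so the trap stays still until triggered.
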(event OnComponentBeginOverlap(Box)
  (params (OverlappedComponent :type Primitive%20Component%20Object%20Reference) (OtherActor :type Actor%20Object%20Reference) (OtherComp :type Primitive%20Component%20Object%20Reference) (OtherBodyIndex :type Integer) (bFromSweep :type Boolean) (SweepResult :type Hit%20Result%20Structure%20%28by%20ref%29))
  (if (== OtherComp (Variables|/Script/Engine.Character|GetCapsuleComponent (Game|GetPlayerCharacter 0)))
    (Class|PaperFlipbookComponent|SetPlaybackPositioninFrames (Variables|Default|GetPaperFlipbook) 0 false)
    (Audio|Components|Audio|Play (Variables|Default|GetPaperFlipbook))
    (Components|Timeline|SetLooping (Variables|Default|GetPaperFlipbook) false)
    (Game|Damage|ApplyDamage OtherActor 1e+01 0 0)))

(fn ConstructionScript
  (Audio|Components|Audio|Stop (Variables|Default|GetPaperFlipbook)))