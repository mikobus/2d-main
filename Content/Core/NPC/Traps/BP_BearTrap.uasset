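; BP_BearTrap is a one-shot flipbook-animated trap that hurts the player.
; When its Box begins an overlap and player 0's location is within a 5-unit tolerance of the trap's, it applies damage, plays a snap sound and starts the non-looping flipbook.
; The trap destroys itself when the animation finishes, or upon taking any damage, in which case it first spawns a BP_DamageInd showing the amount.
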(event OnComponentBeginOverlap(Box)
  (params (OverlappedComponent :type Primitive%20Component%20Object%20Reference) (OtherActor :type Actor%20Object%20Reference) (OtherComp :type Primitive%20Component%20Object%20Reference) (OtherBodyIndex :type Integer) (bFromSweep :type Boolean) (SweepResult :type Hit%20Result%20Structure%20%28by%20ref%29))
  (if (Utilities|Operators|EqualEqual (Transformation|GetActorLocation (Game|GetPlayerCharacter 0)) (Transformation|GetActorLocation) 5.0)
    (Game|Damage|ApplyDamage (Game|GetPlayerCharacter 0) 2.0 0 0)
    (Audio|PlaySoundatLocation "/Game/Core/assets/Audio/bear-trap-103800.bear-trap-103800" (Transformation|GetActorLocation) "0, 0, 0" 1.0 1.0 0.0 0 0 0 0)
    (Audio|Components|Audio|Play (Variables|Default|GetPaperFlipbook))))

(event OnFinishedPlaying(PaperFlipbook)
  (Actor|DestroyActor))

(event EventBeginPlay)

(event Game|Damage|EventAnyDamage
  (params (Damage :type Float%20%28single-precision%29) (DamageType :type Damage%20Type%20Object%20Reference) (InstigatedBy :type Controller%20Object%20Reference) (DamageCauser :type Actor%20Object%20Reference))
  (Game|SpawnActorfromClass "/Game/Core/Interface/DamageIndicators/BP_DamageInd.BP_DamageInd_C" (Math|Transform|MakeTransform (Transformation|GetActorLocation) "0, 0, 0" "1.000000,1.000000,1.000000") "Undefined" "MultiplyWithRoot" 0 Damage "" 0)
  (Actor|DestroyActor))

(fn ConstructionScript
  (Audio|Components|Audio|Stop (Variables|Default|GetPaperFlipbook))
  (Components|Timeline|SetLooping (Variables|Default|GetPaperFlipbook) false))