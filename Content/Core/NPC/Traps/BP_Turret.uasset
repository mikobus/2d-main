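; BP_Turret is a tile-grid trap NPC that fires projectiles left and right in a repeating cycle while on screen.
; It pre-spawns a projectile pool at BeginPlay, then reuses idle entries for each shot.
; MovementTick steps through charge, mark and delay flags before firing and playing the flipbook.
; The turret destroys itself and its pool once it falls over 20 tiles behind the player.
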(event OnFinishedPlaying(PaperFlipbook)
  (Sprite|SetFlipbook (Variables|Default|GetPaperFlipbook) "/Game/Core/Spirtes/Traps/IdleTurret.IdleTurret"))

(event Game|Damage|EventAnyDamage
  (params (Damage :type Float%20%28single-precision%29) (DamageType :type Damage%20Type%20Object%20Reference) (InstigatedBy :type Controller%20Object%20Reference) (DamageCauser :type Actor%20Object%20Reference)))

(event EventMovementTick
  (bind _returnvalue (Viewport|GetViewportSize))
  (CallFunction|FindPlayer)
  (bind (_tilex _tiley) (Default|TiletoLocation (Variables|Default|GetTile%20Map) (Variables|Default|GetOur%20Left/%20Right) (Variables|Default|GetOur%20Up/%20Down)))
  (if (< (Variables|Default|GetOur%20Up/%20Down) (- (Variables|Default|GetPlayer%20Up/%20Down) 20))
    (for _array_element (Variables|Default|GetProjectilePool)
      (Actor|DestroyActor _array_element))
    (Actor|DestroyActor)
    (elif (and (Variables|Default|GetAttackCharged?) (Math|Boolean|ANDBoolean (> (.x (.ScreenLocation (Class|PlayerController|ProjectWorldLocationtoScreen (Game|GetPlayerController 0) (Math|Vector|MakeVector _tilex _tiley 5.0) false))) 0.0) (> (.y (.ScreenLocation (Class|PlayerController|ProjectWorldLocationtoScreen (Game|GetPlayerController 0) (Math|Vector|MakeVector _tilex _tiley 5.0) false))) 0.0) (< (.x (.ScreenLocation (Class|PlayerController|ProjectWorldLocationtoScreen (Game|GetPlayerController 0) (Math|Vector|MakeVector _tilex _tiley 5.0) false))) (.x _returnvalue)) (< (.y (.ScreenLocation (Class|PlayerController|ProjectWorldLocationtoScreen (Game|GetPlayerController 0) (Math|Vector|MakeVector _tilex _tiley 5.0) false))) (.y _returnvalue))))
      (if (Variables|Default|GetAttackMarked?)
        (if (Variables|Default|GetThirdDelay)
          (Audio|Components|Audio|Play (Variables|Default|GetPaperFlipbook))
          (Components|Timeline|SetLooping (Variables|Default|GetPaperFlipbook) false)
          (CallFunction|SpawnLeftProjectile)
          (CallFunction|SpawnRightProjectile)
          (Variables|Default|SetAttackMarked? false)
          (Variables|Default|SetAttackCharged? false)
          (Variables|Default|SetThirdDelay false)
          (else
            (Variables|Default|SetThirdDelay true)))
        (else
          (Variables|Default|SetAttackMarked? true)))
      (else
        (Sprite|SetFlipbook (Variables|Default|GetPaperFlipbook) "/Game/Core/Spirtes/Traps/Turret_Spritesheet1-Sheet1.Turret_Spritesheet1-Sheet1")
        (Class|PaperFlipbookComponent|SetPlaybackPositioninFrames (Variables|Default|GetPaperFlipbook) 3 false)
        (Audio|Components|Audio|Stop (Variables|Default|GetPaperFlipbook))
        (Variables|Default|SetAttackCharged? true)))))

(event EventBeginPlay
  (bind _arrow1 (Variables|Default|GetArrow1))
  (bind _returnvalue (Transformation|GetWorldLocation _arrow1))
  (Utilities|FlowControl|Delay 0.2)
  (|CallParentFunction)
  (CallFunction|SetinUse true)
  (for _index (range 0 10)
    (bind _returnvalue_2 (Game|SpawnActorfromClass "/Game/Core/Items/Projectiles/SpellEffects/Turret_Projectile.Turret_Projectile_C" (Math|Transform|MakeTransform (Math|Vector|MakeVector (.x _returnvalue) (.y _returnvalue) 5.0) "0, 0, 0" "1.000000,1.000000,1.000000") "Undefined" "MultiplyWithRoot" 0 (Variables|Default|GetOnRightSide) (Variables|Default|GetOnLeftSide) 1.0 "Friendly" 0))
    (Utilities|Array|Add (Variables|Default|GetProjectilePool) _returnvalue_2)))

(fn ConstructionScript)

(fn FirstAvailableProjectile
  (for _array_element (Variables|Default|GetProjectilePool)
    (Utilities|IsValid _array_element
      (:Is%20Valid
        (if (not (Variables|/Game/Core/NPC/BP_Enemy.BP_Enemy_C|GetInUse _array_element))
          (return _array_element))))))

(fn SpawnLeftProjectile
  (bind _paperflipbook (Variables|Default|GetPaperFlipbook))
  (bind _returnvalue (Transformation|GetWorldLocation _paperflipbook))
  (bind _array_element (CallFunction|FirstAvailableProjectile))
  (Utilities|IsValid _array_element
    (:Is%20Valid
      (Variables|/Game/Core/Items/Projectiles/SpellEffects/Turret_Projectile.Turret_Projectile_C|SetShootLeft _array_element true)
      (Variables|/Game/Core/Items/Projectiles/SpellEffects/Turret_Projectile.Turret_Projectile_C|SetShootRight _array_element false)
      (Transformation|SetWorldRotation (Variables|/Game/Core/NPC/BP_Enemy.BP_Enemy_C|GetPaperFlipbook _array_element) "0.000000,0.000000,90.000000" false false)
      (Default|CheckDirection _array_element)
      (Transformation|SetActorLocation _array_element (Math|Vector|MakeVector (.x _returnvalue) (- (.y _returnvalue) 32.0) 5.0) false false)
      (Default|SetinUse _array_element true)
      (Default|FindPlayer _array_element)
      (return _array_element))))

(fn SpawnRightProjectile
  (bind _paperflipbook (Variables|Default|GetPaperFlipbook))
  (bind _returnvalue (Transformation|GetWorldLocation _paperflipbook))
  (bind _array_element (CallFunction|FirstAvailableProjectile))
  (Variables|/Game/Core/Items/Projectiles/SpellEffects/Turret_Projectile.Turret_Projectile_C|SetShootRight _array_element true)
  (Variables|/Game/Core/Items/Projectiles/SpellEffects/Turret_Projectile.Turret_Projectile_C|SetShootLeft _array_element false)
  (Transformation|SetWorldRotation (Variables|/Game/Core/NPC/BP_Enemy.BP_Enemy_C|GetPaperFlipbook _array_element) "0.000000,-180.000000,90.000000" false false)
  (Utilities|IsValid _array_element
    (:Is%20Valid
      (Default|CheckDirection _array_element)
      (Transformation|SetActorLocation _array_element (Math|Vector|MakeVector (.x _returnvalue) (+ (.y _returnvalue) 32.0) 5.0) false false)
      (Default|SetinUse _array_element true)
      (Default|FindPlayer _array_element)
      (return _array_element))))