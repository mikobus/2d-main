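; Trigger-driven spawner that scatters items or other actors across random dungeon tilemap locations.
; When the player overlaps its box, it disables the box, swaps the tile at the trigger coordinates (opening the door) and starts the Spawn timer.
; Each Spawn call box-traces a random tile for free space, then spawns ClassToSpawn, or for BP_Item a random DTItems row with a random value, decrementing ActorsToSpawn.
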(event OnComponentBeginOverlap(Box)
  (params (OverlappedComponent :type Primitive%20Component%20Object%20Reference) (OtherActor :type Actor%20Object%20Reference) (OtherComp :type Primitive%20Component%20Object%20Reference) (OtherBodyIndex :type Integer) (bFromSweep :type Boolean) (SweepResult :type Hit%20Result%20Structure%20%28by%20ref%29))
  ;[0.15 0.15 0.15 0.5] Actor Spawn Loop
  ;;[0.15 0.15 0.15 0.5] open the door
  (if (== OtherActor (Game|GetPlayerCharacter 0))
    (Utilities|Time|SetTimerbyFunctionName 0 "Spawn" 0.01 (Variables|Default|GetLooping))
    (Collision|SetCollisionEnabled (Variables|Default|GetBox) "NoCollision")
    (Class|PaperTileMapComponent|SetTile (Variables|/Game/Core/Grid/Level/BP_TIleMapGrid.BP_TIleMapGrid_C|GetTileMap (Variables|Default|GetTile%20Map)) (Variables|Default|GetTriggerLocationLeftRight) (Variables|Default|GetTriggerLocationUpDown) 0 (Utilities|Struct|MakePaperTileInfo 41 "/Game/Core/Tilemaps/tileset_dungeon_TileSet1.tileset_dungeon_TileSet1" false true false))))

(event Custom|Spawn
  (bind _spawnspace (Variables|Default|GetSpawnSpace))
  ;[0.15 0.15 0.15 0.5] Actor Spawn Loop
  (if (<= (Variables|Default|GetActorsToSpawn) 0)
    (Variables|Default|SetLooping false)
    (else
      (bind (_tilex _tiley) (Default|TiletoLocation (Variables|Default|GetTile%20Map) (Math|Random|RandomIntegerinRange 1 22) (Math|Random|RandomIntegerinRange (Variables|Default|GetMinSpawnHeight) (Variables|Default|GetMaxSpawnHeight))))
      (bind _returnvalue (Collision|BoxTraceByChannel (Math|Vector|MakeVector _tilex _tiley 5.0) (Math|Vector|MakeVector _tilex _tiley 5.0) (Math|Vector|MakeVector _spawnspace _spawnspace 5.0) "0, 0, 0" "TraceTypeQuery1" false 0 "Persistent"))
      (if (not _returnvalue)
        (if (== (Variables|Default|GetClassToSpawn) "/Game/Core/Inventory/Blueprints/BP_Item.BP_Item_C")
          (CallFunction|SpawnItemObject 0.0 0.0)
          (else
            (CallFunction|SpawnNormalObject 0.0 0.0)))
        (Variables|Default|SetActorsToSpawn (- (Variables|Default|GetActorsToSpawn) 1))))))

(event EventBeginPlay
  ;[0.15 0.15 0.15 0.5] Timer
  (Development|PrintString "Spawn")
  (Utilities|FlowControl|Delay 0.2)
  (Utilities|FlowControl|Sequence
    (:then_0
      (bind _asbp_gamemode (Utilities|Casting|CastToBP_Gamemode (Game|GetGameMode)))
      (Variables|Default|SetTile%20Map (Default|GetTIlemap _asbp_gamemode)))
    (:then_1
      ;[0.15 0.15 0.15 0.5] set desired spawner location
      (bind (_tilex _tiley) (Default|TiletoLocation (Variables|Default|GetTile%20Map) (Variables|Default|GetTriggerLocationLeftRight) (Variables|Default|GetTriggerLocationUpDown))))))

(fn ConstructionScript)

(fn SpawnNormalObject
  (params (Tile%20X :type Float%20%28double-precision%29) (Tile%20Y :type Float%20%28double-precision%29))
  ;[0.15 0.15 0.15 0.5] Spawn Normal Object (weapon, equip..)
  (Game|SpawnActorfromClass (Variables|Default|GetClassToSpawn) (Math|Transform|MakeTransform (Math|Vector|MakeVector Tile%20X Tile%20Y 5.0) "0, 0, 0" "1.000000,1.000000,1.000000") "Undefined" "MultiplyWithRoot" 0 0))

(fn SpawnItemObject
  (params (Tile%20X :type Float%20%28double-precision%29) (Tile%20Y :type Float%20%28double-precision%29))
  (bind _dt_items (Variables|Default|GetDT_Items))
  ;[0.15 0.15 0.15 0.5] Spawn Item Object (gold, charm...)
  ;;[0.15 0.15 0.15 0.5] get all possible items (DT rows)
  (bind _outrownames (DataTable|GetDataTableRowNames _dt_items))
  ;;[0.15 0.15 0.15 0.5] get row of random item
  (bind _returnvalue (Utilities|GetDataTableRow _dt_items (.OutItem (Utilities|Array|Random _outrownames)))
    (:then
      (Game|SpawnActorfromClass "/Game/Core/Inventory/Blueprints/BP_Item.BP_Item_C" (Math|Transform|MakeTransform (Math|Vector|MakeVector Tile%20X Tile%20Y 5.0) "0, 0, 0" "1.000000,1.000000,1.000000") "Undefined" "MultiplyWithRoot" 0 _returnvalue (.animation (Utilities|Struct|BreakS_Item _returnvalue)) (Math|Random|RandomIntegerinRange 1 10) 0)
      ;;[0.15 0.15 0.15 0.5] get item type
      (switch Utilities|FlowControl|Switch|SwitchonE_ItemTypes (.BP_type (Utilities|Struct|BreakS_Item _returnvalue))))))