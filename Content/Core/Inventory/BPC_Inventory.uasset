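; Inventory component that lets the player pick up weapons and shows them in an inventory widget.
; E sphere-traces at the player's location; a hit BP_Weapon is stored and its actor destroyed, unless nine weapons are held.
; With no active weapon, the pickup fills the widget's weapon slot and is equipped on BP_Character; otherwise AddWeapon appends it and refreshes the widget.
; Tab toggles the widget and mouse cursor.
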(event EventBeginPlay
  (bind _returnvalue (UserInterface|CreateWidget "/Game/Core/Inventory/InventoryUI.InventoryUI_C"))
  (bind _output_get (Variables|Default|SetInventoryReference _returnvalue))
  (UserInterface|Viewport|AddtoViewport _output_get 0))

(event Input|KeyboardEvents|Tab
  (params (Key :type Key%20Structure :default "None"))
  (bind _inventoryreference (Variables|Default|GetInventoryReference))
  (:Pressed
    (if (Widget|IsVisible (Variables|Default|GetInventoryReference))
      (Widget|SetVisibility _inventoryreference "Hidden")
      (Variables|/Script/Engine.PlayerController|SetbShowMouseCursor (Game|GetPlayerController (Variables|/Script/Engine.Pawn|GetPlayerState (Game|GetPlayerCharacter 0))) false)
      (else
        (Widget|SetVisibility _inventoryreference "Visible")
        (Variables|/Script/Engine.PlayerController|SetbShowMouseCursor (Game|GetPlayerController (Variables|/Script/Engine.Pawn|GetPlayerState (Game|GetPlayerCharacter 0))) true)))))

(event Input|KeyboardEvents|E
  (params (Key :type Key%20Structure :default "None"))
  (bind _returnvalue (Game|GetPlayerCharacter 0))
  (bind _returnvalue_2 (Transformation|GetActorLocation _returnvalue))
  (:Pressed
    (bind (_outhit _returnvalue_3) (Collision|SphereTraceByChannel _returnvalue_2 _returnvalue_2 32.0 "TraceTypeQuery1" false (Utilities|Array|MakeArray _returnvalue) "None"))
    (if (>= (Utilities|Array|Length (Variables|Default|GetWeaponArray)) 9)
      (Development|PrintString "Inventory Full")
      (elif _returnvalue_3
        (bind _asbp_weapon (Utilities|Casting|CastToBP_Weapon (.hitactor _outhit)))
        (Development|PrintString (Utilities|String|ToString(Name) (.rowname (Utilities|Struct|BreakS_Slots (Variables|/Game/Core/Inventory/InventoryUI.InventoryUI_C|GetActiveWeapon (Variables|Default|GetInventoryReference))))))
        ;[0.15 0.15 0.15 0.5] active weapon exists?
        (Utilities|IsValid (.datatable (Utilities|Struct|BreakS_Slots (Variables|/Game/Core/Inventory/InventoryUI.InventoryUI_C|GetActiveWeapon (Variables|Default|GetInventoryReference))))
          (:Is%20Valid
            ;[0.15 0.15 0.15 0.5] add to inventory
            (CallFunction|AddWeapon (Variables|/Game/Core/Weapons/BP_Weapon.BP_Weapon_C|GetItemData _asbp_weapon)))
          (:Is%20Not%20Valid
            ;[0.15 0.15 0.15 0.5] add to active weapon and inventory
            (Default|AddtoSlot (Variables|/Game/Core/Inventory/InventoryUI.InventoryUI_C|GetWeapon (Variables|Default|GetInventoryReference)) (Variables|/Game/Core/Weapons/BP_Weapon.BP_Weapon_C|GetItemData _asbp_weapon))
            (Variables|/Game/Core/Inventory/InventoryUI.InventoryUI_C|SetActiveWeapon (Variables|Default|GetInventoryReference) (Variables|/Game/Core/Weapons/BP_Weapon.BP_Weapon_C|GetItemData _asbp_weapon))
            (bind _asbp_character (Utilities|Casting|CastToBP_Character (Game|GetPlayerCharacter 0)))
            (Default|EquipWeapon _asbp_character (Variables|/Game/Core/Weapons/BP_Weapon.BP_Weapon_C|GetItemData _asbp_weapon))))
        (Actor|DestroyActor (.hitactor _outhit))))))

(event Input|KeyboardEvents|Escape
  (params (Key :type Key%20Structure :default "None")))

(fn AddWeapon
  (params (NewWeapon :type S%20Slots%20Structure%20%28by%20ref%29))
  (if (not (>= (Utilities|Array|Length (Variables|Default|GetWeaponArray)) 9))
    (Utilities|Array|Add (Variables|Default|GetWeaponArray) NewWeapon)
    (Default|UpdateInventory (Variables|Default|GetInventoryReference) self)))